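; Player controller that toggles the pause menu from the PauseMenu input action.
; Opening pauses the game, shows the cursor, sets Game and UI input, then creates the pause widget and plays its animation forward.
; The controller keeps the widget reference and closes it through the widget's own RemovePauseMenu.
; A two-value CurrentState is initialized on BeginPlay, but its toggle logic is disconnected.
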(event EventBeginPlay
  (Variables|Default|SetCurrent%20State "NewEnumerator0"))

(event EventTick
  (params (DeltaSeconds :type Float%20%28single-precision%29)))

(event Input|ActionEvents|InputActionPauseMenu
  (params (Key :type Key%20Structure :default "None"))
  ;[1 0.6234 0.4637] PAUSE MENU
  (:Pressed
    (if (Variables|Default|GetisPauseMenuOn)
      (Variables|Default|SetisPauseMenuOn false)
      (Default|RemovePauseMenu (stale _returnvalue))
      (else
        (Variables|Default|SetisPauseMenuOn true)
        (bind _returnvalue (CallFunction|PauseMenuOpen))))))

(fn ConstructionScript)

(fn PauseMenuOpen
  ;[1 0.6234 0.4637] change the settings
  (Game|SetGamePaused true)
  (Variables|Default|SetbShowMouseCursor true)
  (Input|SetInputModeGameandUI self 0 "DoNotLock" true)
  ;[1 0.6234 0.4637] stop the game and start the animation
  (bind _returnvalue (UserInterface|CreateWidget "/Game/Assets/UI_Assets/Widgets/PauseMenu_Widget.PauseMenu_Widget_C"))
  (UserInterface|Viewport|AddtoViewport _returnvalue 0)
  (Default|PlayAnimationForward _returnvalue)
  (return _returnvalue))