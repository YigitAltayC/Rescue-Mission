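; BP_CharacterData is a data-holder Blueprint that stores current and max health for the player's normal (Metroid) and mutated forms.
; Each form has its own health struct, read through separate getter functions.
; SetPlayerHealth writes both values to one of the structs, chosen by an IsMutated flag.
; It has no active event or construction logic and does no clamping.
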(event EventBeginPlay)

(event Collision|EventActorBeginOverlap
  (params (OtherActor :type Actor%20Object%20Reference)))

(event EventTick
  (params (DeltaSeconds :type Float%20%28single-precision%29)))

(fn ConstructionScript)

(fn GetNormalPlayerCurrentHealth
  (return (.health (Variables|Default|GetMetroid%20Character%20Health%20Data))))

(fn GetMutatedPlayerCurrentHealth
  (return (.health (Variables|Default|GetMutated%20Character%20Health%20Data))))

(fn GetNormalPlayerMaxHealth
  (return (.maxhealth (Variables|Default|GetMetroid%20Character%20Health%20Data))))

(fn GetMutatedPlayerMaxHealth
  (return (.maxhealth (Variables|Default|GetMutated%20Character%20Health%20Data))))

(fn SetPlayerHealth
  (params (Health :type Float%20%28double-precision%29) (Max%20Health :type Float%20%28double-precision%29) (Is%20Mutated :type Boolean))
  (LocalVariables|SetLocal%20Health Health)
  (LocalVariables|SetMax%20Local%20Health Max%20Health)
  (if Is%20Mutated
    (Variables|Default|SetMutated%20Character%20Health%20Data (Utilities|Struct|MakeController_Data (LocalVariables|GetLocal%20Health) (LocalVariables|GetMax%20Local%20Health)))
    (else
      (Variables|Default|SetMetroid%20Character%20Health%20Data (Utilities|Struct|MakeController_Data (LocalVariables|GetLocal%20Health) (LocalVariables|GetMax%20Local%20Health))))))