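; Playable mutated form (Bringer of Death) of the 2D side-scrolling player, with movement, jump, melee attack and spawned spell cast.
; Tick locks Y, selects flipbooks from velocity and action flags, and flips facing through control rotation.
; Sprite overlaps during attacks damage enemies, while damage taken is copied to the Metroid character's Health.
; M hands possession and position back to that character behind a black fade, then parks this one at a fixed location.
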(event OnComponentBeginOverlap(Sprite)
  (params (OverlappedComponent :type Primitive%20Component%20Object%20Reference) (OtherActor :type Actor%20Object%20Reference) (OtherComp :type Primitive%20Component%20Object%20Reference) (OtherBodyIndex :type Integer) (bFromSweep :type Boolean) (SweepResult :type Hit%20Result%20Structure%20%28by%20ref%29))
  (bind _asenemy_blueprint (Utilities|Casting|CastToEnemyBlueprint OtherActor))
  (if (and (Variables|Default|GetIs%20Attacking) (== (Class|PaperFlipbookComponent|GetFlipbook (Variables|Default|GetSprite)) "/Game/Assets/Enemy_Assets/Bringer-Of-Death/Individual_Sprite/Attack/Bringer-of-Death-Character-Attack.Bringer-of-Death-Character-Attack"))
    (Game|Damage|ApplyDamage _asenemy_blueprint (Variables|Default|GetBase%20Damage) 0 0)))

(event OnComponentEndOverlap(CapsuleComponent)
  (params (OverlappedComponent :type Primitive%20Component%20Object%20Reference) (OtherActor :type Actor%20Object%20Reference) (OtherComp :type Primitive%20Component%20Object%20Reference) (OtherBodyIndex :type Integer))
  ;[1 1 1] This part is unnecessary at the moment
)

(event Custom|Spawn%20Spell
  (bind _returnvalue (Transformation|GetActorTransform))
  (if (Variables|Default|GetIs%20Moving%20Right)
    (Variables|Default|SetSpell%20Cast%20Distance 1e+02)
    (else
      (Variables|Default|SetSpell%20Cast%20Distance -1e+02)))
  (Game|SpawnActorfromClass "/Game/Blueprints/Bullet_and_Impact_Blueprint/Cast/BP_MutatedCast.BP_MutatedCast_C" (Math|Transform|MakeTransform (Math|Vector|MakeVector (+ (.x (.location _returnvalue)) (Variables|Default|GetSpell%20Cast%20Distance)) (.y (.location _returnvalue)) (+ (.z (.location _returnvalue)) 25.0)) (.rotation _returnvalue) (.scale _returnvalue)) "Undefined" 0 0)
  (Utilities|FlowControl|Delay 1.0))

(event Custom|Handle%20Animation
  (if (> (Math|Vector|VectorLength (Variables|/Script/Engine.MovementComponent|GetVelocity (Variables|Character|GetCharacterMovement))) 0.0)
    (Sprite|SetFlipbook (Variables|Default|GetSprite) "/Game/Assets/Enemy_Assets/Bringer-Of-Death/Individual_Sprite/Walk/Bringer-of-Death_Walk.Bringer-of-Death_Walk")
    (elif (Variables|Default|GetIs%20Attacking)
      (Sprite|SetFlipbook (Variables|Default|GetSprite) "/Game/Assets/Enemy_Assets/Bringer-Of-Death/Individual_Sprite/Attack/Bringer-of-Death-Character-Attack.Bringer-of-Death-Character-Attack")
      (elif (Variables|Default|GetIs%20Casting)
        (Sprite|SetFlipbook (Variables|Default|GetSprite) "/Game/Assets/Enemy_Assets/Bringer-Of-Death/Individual_Sprite/Cast/Bringer-of-Death_Cast.Bringer-of-Death_Cast")
        (else
          (Sprite|SetFlipbook (Variables|Default|GetSprite) "/Game/Assets/Enemy_Assets/Bringer-Of-Death/Individual_Sprite/Idle/Bringer-of-Death_Idle.Bringer-of-Death_Idle"))))))

(event Custom|CustomEvent
  ;[1 0.6234 0.4637] MUTATION
  (Widget|RemovefromParent (stale Input|KeyboardEvents|M _returnvalue_2)))

(event Custom|Stuck%20Y
  (bind _returnvalue (Transformation|GetActorLocation))
  ;[1 1 1] Make sure player has correct y axis
  (if (not (== (.y (Transformation|GetWorldLocation (Variables|Default|GetSprite self))) -1.9e+02))
    (Transformation|SetActorLocation (Math|Vector|MakeVector (.x _returnvalue) -1.9e+02 (.z _returnvalue)) false false)))

(event EventBeginPlay
  (bind _returnvalue (Actor|GetActorOfClass "/Game/Blueprints/Chracter_Blueprint/Paper2DCharacter.Paper2DCharacter_C"))
  (Variables|Default|SetMetroid _returnvalue))

(event EventTick
  (params (DeltaSeconds :type Float%20%28single-precision%29))
  (if (not (Variables|Default|GetSwitched%20to%20Metroid%20))
    (Variables|Default|SetJumpMaxCount self 1)
    (CallFunction|StuckY)
    (CallFunction|HandleAnimation)
    (CallFunction|HandlePlayerRotation)))

(event Game|Damage|EventAnyDamage
  (params (Damage :type Float%20%28single-precision%29) (DamageType :type Damage%20Type%20Object%20Reference) (InstigatedBy :type Controller%20Object%20Reference) (DamageCauser :type Actor%20Object%20Reference))
  ;[1 1 1] Player Taking Damage
  (bind _output_get (Variables|Default|SetHealth (Math|Float|Clamp(Float) (- (Variables|Default|GetHealth) Damage) 0.0 (Variables|Default|GetDefault%20Health))))
  (Variables|/Game/Blueprints/Chracter_Blueprint/Paper2DCharacter.Paper2DCharacter_C|SetHealth (Variables|Default|GetMetroid) _output_get)
  (if (and (<= (Variables|Default|GetHealth) 0.0) (not (Variables|Default|GetIs%20Dead)))
    (Variables|Default|SetIs%20Dead true)
    (CallFunction|PlayerDeath)))

(event Collision|EventActorBeginOverlap
  (params (OtherActor :type Actor%20Object%20Reference)))

(event Input|ActionEvents|InputActionFireGun
  (params (Key :type Key%20Structure :default "None"))
  (bind _sprite (Variables|Default|GetSprite))
  (:Pressed
    (if (and (not (Variables|Default|GetIs%20Attacking)) (not (Variables|Default|GetIs%20Casting)))
      (Variables|Default|SetIs%20Attacking true)))
  (:Released
    (if (Variables|Default|GetIs%20Attacking)
      (Utilities|FlowControl|Delay (- (Class|PaperFlipbookComponent|GetFlipbookLength _sprite) (Components|Timeline|GetPlaybackPosition _sprite)))
      (Variables|Default|SetIs%20Attacking false))))

(event Input|ActionEvents|InputActionSecondaryAttack
  (params (Key :type Key%20Structure :default "None"))
  (bind _sprite (Variables|Default|GetSprite))
  (:Pressed
    (if (and (not (Variables|Default|GetIs%20Attacking)) (not (Variables|Default|GetIs%20Casting)))
      (Variables|Default|SetIs%20Casting true)
      (Sprite|SetFlipbook (Variables|Default|GetSprite) "/Game/Assets/Enemy_Assets/Bringer-Of-Death/Individual_Sprite/Cast/Bringer-of-Death_Cast.Bringer-of-Death_Cast")
      (CallFunction|SpawnSpell)))
  (:Released
    (if (Variables|Default|GetIs%20Casting)
      (Utilities|FlowControl|Delay (- (Class|PaperFlipbookComponent|GetFlipbookLength _sprite) (Components|Timeline|GetPlaybackPosition _sprite)))
      (Variables|Default|SetIs%20Casting false)
      (Sprite|SetFlipbook (Variables|Default|GetSprite) "/Game/Assets/Enemy_Assets/Bringer-Of-Death/Individual_Sprite/Idle/Bringer-of-Death_Idle.Bringer-of-Death_Idle"))))

(event Input|ActionEvents|InputActionJump
  (params (Key :type Key%20Structure :default "None"))
  (:Pressed
    ;[1 1 1] Jumping
    (Character|Jump))
  (:Released
    (Character|StopJumping)))

(event Input|AxisEvents|InputAxisMovement
  (params (AxisValue :type Float%20%28single-precision%29))
  ;[1 1 1] Movement
  (if (not (Variables|Default|GetIs%20Attacking))
    (Pawn|Input|AddMovementInput "1.000000, 0,0.000000" AxisValue false)
    ;;[1 1 1] Set the Movement Direction According to Axis
    (if (> AxisValue 0.0)
      (Variables|Default|SetIs%20Moving%20Right true)
      (elif (< AxisValue 0.0)
        (Variables|Default|SetIs%20Moving%20Right false)))))

(event Input|KeyboardEvents|M
  (params (Key :type Key%20Structure :default "None"))
  ;[1 0.6234 0.4637] MUTATION
  (:Pressed
    (bind _returnvalue (Actor|GetActorOfClass "/Game/Blueprints/Chracter_Blueprint/Paper2DCharacter.Paper2DCharacter_C"))
    (Variables|/Game/Blueprints/Chracter_Blueprint/Paper2DCharacter.Paper2DCharacter_C|SetHealth _returnvalue (Variables|Default|GetHealth))
    (CameraFades|StartCameraFade (Game|GetPlayerCameraManager 0) 0.0 1.0 1.0 "(R=0.000000,G=0.000000,B=0.000000,A=1.000000)" false true)
    (bind _returnvalue_2 (UserInterface|CreateWidget "/Game/BlackScreen.BlackScreen_C"))
    (UserInterface|Viewport|AddtoViewport _returnvalue_2 0)
    (Utilities|Time|SetTimerbyEvent (delegate Custom|CustomEvent) 1.0)
    (Transformation|SetActorLocation _returnvalue (Transformation|GetActorLocation (Game|GetPlayerCharacter 0)) false false)
    (Pawn|Possess (Game|GetPlayerController 0) _returnvalue)
    (Variables|/Game/Blueprints/Chracter_Blueprint/Paper2DCharacter.Paper2DCharacter_C|SetSwitched%20to%20Mutation _returnvalue false)
    (Variables|Default|SetSwitched%20to%20Metroid%20 true)
    (Transformation|SetActorLocation "-5237.000000,-190.000000,-604.000000" false false)
    (CameraFades|StartCameraFade (Game|GetPlayerCameraManager 0) 1.0 0.0 1.0 "(R=0.000000,G=0.000000,B=0.000000,A=1.000000)" false false)
    (Utilities|FlowControl|Delay 1.0)))

(fn ConstructionScript
  (|CallParentFunction))

(fn HandlePlayerRotation
  (Math|Float|CompareFloat (.x (Variables|/Script/Engine.MovementComponent|GetVelocity (Variables|Character|GetCharacterMovement))) 0.0
    (:>
      (Pawn|SetControlRotation (Pawn|GetController) (Math|Rotator|MakeRotator 0.0 0.0 0.0) :!label _label))
    (:==
      (if (Variables|Default|GetIs%20Moving%20Right)
        (goto _label)
        (else
          (Pawn|SetControlRotation (Pawn|GetController) (Math|Rotator|MakeRotator 0.0 0.0 1.8e+02) :!label _label_2))))
    (:<
      (goto _label_2))))

(fn MutatedPlayerRef
  (return 0))