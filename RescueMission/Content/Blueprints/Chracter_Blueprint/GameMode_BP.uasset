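; Game mode that handles persistence: player position, boss defeat state, collected potions and sound volumes.
; BeginPlay loads or creates the "save" and "inventory" slots, destroys stored potion actors, replaces dead Golem and Demon bosses with corpses, and applies saved sound-mix volumes.
; Save records position and boss states, resets player health to default and writes the "save" slot.
; Both slots share one SaveGame variable, so the inventory object replaces the main one after BeginPlay.
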(event Custom|Save
  (CallFunction|SavePlayerPosition)
  (CallFunction|SaveBossesState)
  (CallFunction|LoadAreBossesAlive)
  (CallFunction|UpdateHealth)
  (SaveGame|SaveGametoSlot (Variables|Default|GetSaveGame) "save"))

(event EventBeginPlay
  (CallFunction|CreateandSetSaveGame)
  (CallFunction|CreateandSetSavePotions)
  (CallFunction|SetGameSound))

(event EventTick
  (params (DeltaSeconds :type Float%20%28single-precision%29)))

(fn ConstructionScript)

(fn CreateandSetSaveGame
  (bind _returnvalue (SaveGame|DoesSaveGameExist "save"))
  (if _returnvalue
    (bind _returnvalue_2 (SaveGame|LoadGamefromSlot "save"))
    (bind _assave_game_bp (Utilities|Casting|CastToSaveGame_BP _returnvalue_2))
    (Variables|Default|SetSaveGame _assave_game_bp)
    (CallFunction|SetPlayerPosition)
    (CallFunction|GetBossReferences)
    (CallFunction|LoadAreBossesAlive)
    (else
      (Utilities|FlowControl|Sequence
        (:then_0
          (bind _returnvalue_3 (SaveGame|CreateSaveGameObject "/Game/Blueprints/Chracter_Blueprint/SaveGame_BP.SaveGame_BP_C"))
          (Variables|Default|SetSaveGame _returnvalue_3)
          (CallFunction|SavePlayerPosition)
          (CallFunction|GetBossReferences)
          (CallFunction|LoadAreBossesAlive))
        (:then_1
          (SaveGame|SaveGametoSlot (Variables|Default|GetSaveGame) "save"))))))

(fn SetPlayerPosition
  (Transformation|SetActorTransform (Game|GetPlayerCharacter 0) (Variables|/Game/Blueprints/Chracter_Blueprint/SaveGame_BP.SaveGame_BP_C|GetplayerPos (Variables|Default|GetSaveGame))))

(fn SavePlayerPosition
  (Variables|/Game/Blueprints/Chracter_Blueprint/SaveGame_BP.SaveGame_BP_C|SetplayerPos (Variables|Default|GetSaveGame) (Transformation|GetActorTransform (Game|GetPlayerCharacter 0))))

(fn CreateandSetSavePotions
  (bind _returnvalue (SaveGame|DoesSaveGameExist "inventory"))
  (if _returnvalue
    (bind _returnvalue_2 (SaveGame|LoadGamefromSlot "inventory"))
    (bind _assave_game_bp (Utilities|Casting|CastToSaveGame_BP _returnvalue_2))
    (bind _output_get (Variables|Default|SetSaveGame _assave_game_bp))
    (for _array_element (Variables|/Game/Blueprints/Chracter_Blueprint/SaveGame_BP.SaveGame_BP_C|GetInventoryData _output_get)
      (Utilities|IsValid (.potionreference _array_element)
        (:Is%20Valid
          (Actor|DestroyActor (.potionreference _array_element)))))
    (else
      (bind _returnvalue_3 (SaveGame|CreateSaveGameObject "/Game/Blueprints/Chracter_Blueprint/SaveGame_BP.SaveGame_BP_C"))
      (bind _output_get_2 (Variables|Default|SetSaveGame _returnvalue_3))
      (SaveGame|SaveGametoSlot _output_get_2 "inventory"))))

(fn UpdateHealth
  (bind _aspaper_2dcharacter (Utilities|Casting|CastToPaper2DCharacter (Game|GetPlayerCharacter 0)))
  (Variables|/Game/Blueprints/Chracter_Blueprint/Paper2DCharacter.Paper2DCharacter_C|SetHealth _aspaper_2dcharacter (Variables|/Game/Blueprints/Chracter_Blueprint/Paper2DCharacter.Paper2DCharacter_C|GetDefault%20Health _aspaper_2dcharacter)))

(fn SaveBossesState
  (for (_array_element _array_index) (Variables|Default|GetBossReferences)
    (Utilities|IsValid _array_element
      (:Is%20Valid
        (bind _asbp_boss (Utilities|Casting|CastToBP_Boss _array_element)
          (:then
            (if (<= (Variables|/Game/Blueprints/Enemy_Bluprints/Bosses/BP_Boss.BP_Boss_C|GetHealth _asbp_boss) 0.0)
              (Utilities|Array|SetArrayElem (Variables|Default|GetAreBossesAlive) _array_index false)
              (else
                (Utilities|Array|SetArrayElem (Variables|Default|GetAreBossesAlive) _array_index true))))
          (:CastFailed
            (Utilities|Array|SetArrayElem (Variables|Default|GetAreBossesAlive) _array_index false :!label _label))))
      (:Is%20Not%20Valid
        (goto _label))))
  (Variables|/Game/Blueprints/Chracter_Blueprint/SaveGame_BP.SaveGame_BP_C|SetAreBossesAlive (Variables|Default|GetSaveGame) (Variables|Default|GetAreBossesAlive))
  (SaveGame|SaveGametoSlot (Variables|Default|GetSaveGame) "save")
  (return))

(fn LoadAreBossesAlive
  (if (Utilities|Array|IsNotEmpty (Variables|/Game/Blueprints/Chracter_Blueprint/SaveGame_BP.SaveGame_BP_C|GetAreBossesAlive (Variables|Default|GetSaveGame)))
    (Variables|Default|SetAreBossesAlive (Variables|/Game/Blueprints/Chracter_Blueprint/SaveGame_BP.SaveGame_BP_C|GetAreBossesAlive (Variables|Default|GetSaveGame)))
    (for (_array_element _array_index) (Variables|Default|GetAreBossesAlive)
      (if (not _array_element)
        (Utilities|IsValid (Utilities|Array|Get(acopy) (Variables|Default|GetBossReferences) _array_index)
          (:Is%20Valid
            (switch int _array_index
              (:0
                (Game|SpawnActorfromClass "/Game/Blueprints/Enemy_Bluprints/Bosses/GolemBoss/BP_GolemDeadBody.BP_GolemDeadBody_C" (Math|Transform|MakeTransform (Math|Vector|MakeVector (.x (.Location (Math|Transform|BreakTransform (Transformation|GetActorTransform (Utilities|Array|Get(acopy) (Variables|Default|GetBossReferences) _array_index))))) (- (.y (.Location (Math|Transform|BreakTransform (Transformation|GetActorTransform (Utilities|Array|Get(acopy) (Variables|Default|GetBossReferences) _array_index))))) 4e+01) (- (.z (.Location (Math|Transform|BreakTransform (Transformation|GetActorTransform (Utilities|Array|Get(acopy) (Variables|Default|GetBossReferences) _array_index))))) 2e+01)) "0, 0, 0" "2.000000,2.000000,2.000000") "Undefined" 0 0)
                (Actor|DestroyActor (Utilities|Array|Get(acopy) (Variables|Default|GetBossReferences) _array_index)))
              (:1
                (Game|SpawnActorfromClass "/Game/Blueprints/Enemy_Bluprints/Bosses/DemonBoss/BP_DeadDemon.BP_DeadDemon_C" (Transformation|GetActorTransform (Utilities|Array|Get(acopy) (Variables|Default|GetBossReferences) _array_index)) "Undefined" 0 0)
                (Actor|DestroyActor (Utilities|Array|Get(acopy) (Variables|Default|GetBossReferences) _array_index))))))))))

(fn GetBossReferences
  (bind _bossreferences (Variables|Default|GetBossReferences))
  (bind _returnvalue (Actor|GetActorOfClass "/Game/Blueprints/Enemy_Bluprints/Bosses/GolemBoss/BP_GolemBoss.BP_GolemBoss_C"))
  (Utilities|Array|Add _bossreferences _returnvalue)
  (bind _returnvalue_2 (Actor|GetActorOfClass "/Game/Blueprints/Enemy_Bluprints/Bosses/DemonBoss/BP_Demon.BP_Demon_C"))
  (Utilities|Array|Add _bossreferences _returnvalue_2))

(fn SetGameSound
  ;[0.1672 0.2024 1] volume saving
  (bind _returnvalue (SaveGame|DoesSaveGameExist "settings"))
  (if _returnvalue
    (bind _returnvalue_2 (SaveGame|LoadGamefromSlot "settings"))
    (bind _assave_game_bp (Utilities|Casting|CastToSaveGame_BP _returnvalue_2))
    (Class|GameplayStatics|SetBaseSoundMix "/Game/MusicAndSfx/SoundClass/SoundClassMix.SoundClassMix")
    (Audio|SetSoundMixClassOverride "/Game/MusicAndSfx/SoundClass/SoundClassMix.SoundClassMix" "/Game/MusicAndSfx/SoundClass/PlayerEffectsSoundClass.PlayerEffectsSoundClass" (Utilities|Array|Get(acopy) (Variables|/Game/Blueprints/Chracter_Blueprint/SaveGame_BP.SaveGame_BP_C|GetsoundValues _assave_game_bp) 1) 1.0 1.0 true)
    (Audio|SetSoundMixClassOverride "/Game/MusicAndSfx/SoundClass/SoundClassMix.SoundClassMix" "/Game/MusicAndSfx/SoundClass/BackgroundSoundClass.BackgroundSoundClass" (Utilities|Array|Get(acopy) (Variables|/Game/Blueprints/Chracter_Blueprint/SaveGame_BP.SaveGame_BP_C|GetsoundValues _assave_game_bp)) 1.0 1.0 true)
    (Audio|SetSoundMixClassOverride "/Game/MusicAndSfx/SoundClass/SoundClassMix.SoundClassMix" "/Game/MusicAndSfx/SoundClass/SoundEffectsClass.SoundEffectsClass" (Utilities|Array|Get(acopy) (Variables|/Game/Blueprints/Chracter_Blueprint/SaveGame_BP.SaveGame_BP_C|GetsoundValues _assave_game_bp) 2) 1.0 1.0 true)))