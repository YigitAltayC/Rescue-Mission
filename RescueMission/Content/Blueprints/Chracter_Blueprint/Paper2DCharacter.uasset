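; Player Paper2D character for a side-scroller, locked to one Y plane, with flipbook animation, timed shooting, inventory and debug teleport keys.
; Tick drives facing, animation and trace-based wall sliding for wall jumps.
; Velocity-polled fall damage, damage events and healer overlaps feed Health, leading to a death screen.
; Mutation copies Health to BP_Mutated_Character, possesses it behind a fade, and sets SwitchedToMutation, which gates most logic here.
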(event OnComponentBeginOverlap(CapsuleComponent)
  (params (OverlappedComponent :type Primitive%20Component%20Object%20Reference) (OtherActor :type Actor%20Object%20Reference) (OtherComp :type Primitive%20Component%20Object%20Reference) (OtherBodyIndex :type Integer) (bFromSweep :type Boolean) (SweepResult :type Hit%20Result%20Structure%20%28by%20ref%29))
  ;[1 1 1] Heal Collision detector
  (if (Actor|ActorHasTag OtherActor "Healer")
    (CallFunction|HealTime)
    (CallFunction|StartHeal)))

(event OnComponentEndOverlap(CapsuleComponent)
  (params (OverlappedComponent :type Primitive%20Component%20Object%20Reference) (OtherActor :type Actor%20Object%20Reference) (OtherComp :type Primitive%20Component%20Object%20Reference) (OtherBodyIndex :type Integer))
  ;[1 1 1] Heal Collision detector
  (if (Actor|ActorHasTag OtherActor "Healer")
    (CallFunction|EndHeal)))

(event OnComponentBeginOverlap(collision)
  (params (OverlappedComponent :type Primitive%20Component%20Object%20Reference) (OtherActor :type Actor%20Object%20Reference) (OtherComp :type Primitive%20Component%20Object%20Reference) (OtherBodyIndex :type Integer) (bFromSweep :type Boolean) (SweepResult :type Hit%20Result%20Structure%20%28by%20ref%29))
  ;[1 1 1] This part is unnecessary at the moment
)

(event OnComponentEndOverlap(collision)
  (params (OverlappedComponent :type Primitive%20Component%20Object%20Reference) (OtherActor :type Actor%20Object%20Reference) (OtherComp :type Primitive%20Component%20Object%20Reference) (OtherBodyIndex :type Integer))
  ;[1 1 1] This part is unnecessary at the moment
)

(event Custom|Handle%20Animation
  (bind _sprite (Variables|Default|GetSprite))
  (bind _charactermovement (Variables|Character|GetCharacterMovement))
  ;[1 1 1] Handle Animation
  (if (not (Variables|Default|GetSwitched%20to%20Mutation))
    (if (AI|Components|NavMovement|IsFalling _charactermovement)
      (if (Variables|Wallslide|GetIsWallslide)
        (Sprite|SetFlipbook (Variables|Default|GetSprite) "/Game/Assets/Chracter_Asset/Cling/player-cling1.player-cling1")
        (else
          (Sprite|SetFlipbook (Variables|Default|GetSprite) (select (< (.z (Transformation|GetVelocity)) 0.0) "/Game/Assets/Chracter_Asset/Jump/playerJumpFlipbook.playerJumpFlipbook" "/Game/Assets/Chracter_Asset/Jump/playerJumpFlipbook.playerJumpFlipbook"))))
      (elif (> (Math|Vector|VectorLength (Variables|/Script/Engine.MovementComponent|GetVelocity _charactermovement)) 0.0)
        (if (Variables|Bullet|GetisShooting)
          (Sprite|SetFlipbook _sprite "/Game/Assets/Chracter_Asset/RunShoot/RunShootFlipbook.RunShootFlipbook")
          (else
            (Sprite|SetFlipbook _sprite "/Game/Assets/Chracter_Asset/Run/playerRunFlipbook.playerRunFlipbook")))
        (elif (Variables|Bullet|GetisShooting)
          (Sprite|SetFlipbook _sprite "/Game/Assets/Chracter_Asset/Stand/playerStandFlipbook.playerStandFlipbook")
          (else
            (Sprite|SetFlipbook _sprite "/Game/Assets/Chracter_Asset/Stand/playerStandFlipbook.playerStandFlipbook")))))))

(event Custom|Handle%20Rotation
  ;[1 0.6234 0.4637] Flip Player According To Axis
  (if (not (Variables|Default|GetSwitched%20to%20Mutation))
    (CallFunction|HandlePlayerRotaion)))

(event Custom|Start%20Heal
  ;[1 1 1] Heal timer
  (if (not (Variables|Default|GetSwitched%20to%20Mutation))
    (bind _returnvalue (Utilities|Time|SetTimerbyEvent (delegate Custom|Heal%20Time) 1.0 true))
    (Variables|Default|SetHeal%20Timer _returnvalue)))

(event Custom|Heal%20Time
  ;[1 1 1] Heal timer
  (if (not (Variables|Default|GetSwitched%20to%20Mutation))
    (CallFunction|Heal)))

(event Custom|End%20Heal
  ;[1 1 1] Heal timer
  (if (not (Variables|Default|GetSwitched%20to%20Mutation))
    (Utilities|Time|ClearandInvalidateTimerbyHandle (Variables|Default|GetHeal%20Timer))))

(event Custom|ApplyConstantDamageToPlayer
  (params (functionCallRepeatDuration :type Float%20%28double-precision%29) (DamageAmount :type Float%20%28double-precision%29) (DamageDuration :type Float%20%28double-precision%29))
  ;[1 0.6234 0.4637] Apply Constant Damage To Player
  (if (not (Variables|Default|GetSwitched%20to%20Mutation))
    (Variables|Default|SetcurrentTime 0.0)
    (bind _returnvalue (Utilities|Time|SetTimerbyEvent (delegate Custom|ConsistentDamage) functionCallRepeatDuration true))))

(event Custom|Spawn%20Bullets
  ;[1 0.6234 0.4637] firing bullet every 0.3 seconds when left mouse is pressed
  (if (not (Variables|Default|GetSwitched%20to%20Mutation))
    (if (Variables|Jump|GetisJumping)
      (Variables|Bullet|SetisShooting false)
      (Utilities|Time|ClearandInvalidateTimerbyHandle (Variables|bullet|GetfireBulletEvent))
      (else
        (Variables|Bullet|SetisShooting true)
        ;;[1 1 1] spawns bullet
        (Game|SpawnActorfromClass (Utilities|Array|Get(acopy) (Variables|Bullet|GetbulletTypes) (Variables|bullet|GetselectedBulletIndex)) (Transformation|GetWorldTransform (Variables|Default|GetbulletSpawnPoint)) "Undefined" 0 0)))))

(event Custom|CustomEvent_0
  ;[1 0.6234 0.4637] MUTATION
  (Widget|RemovefromParent (stale Custom|Mutation _returnvalue_2)))

(event Custom|Test%20Shot
  ;[1 1 1] Test Shot
  ;;[1 1 1] spawns bullet
  (Game|SpawnActorfromClass (Utilities|Array|Get(acopy) (Variables|Bullet|GetbulletTypes) (Variables|bullet|GetselectedBulletIndex)) (Transformation|GetWorldTransform (Variables|Default|GetbulletSpawnPoint)) "Undefined" 0 0))

(event Custom|Mutation
  ;[1 0.6234 0.4637] MUTATION
  (bind _returnvalue (Actor|GetActorOfClass "/Game/Blueprints/Chracter_Blueprint/BP_Mutated_Character.BP_Mutated_Character_C"))
  (Variables|Paper2DCharacter_C|SetHealth _returnvalue (Variables|Health|GetHealth))
  (CameraFades|StartCameraFade (Game|GetPlayerCameraManager 0) 0.0 1.0 1.0 "(R=0.000000,G=0.000000,B=0.000000,A=1.000000)" false true)
  (bind _returnvalue_2 (UserInterface|CreateWidget "/Game/BlackScreen.BlackScreen_C"))
  (UserInterface|Viewport|AddtoViewport _returnvalue_2 0)
  (Utilities|Time|SetTimerbyEvent (delegate Custom|CustomEvent_0) 1.0)
  (Transformation|SetActorLocation _returnvalue (Transformation|GetActorLocation (Game|GetPlayerCharacter 0)) false false)
  (Pawn|Possess (Game|GetPlayerController 0) _returnvalue)
  (Variables|/Game/Blueprints/Chracter_Blueprint/BP_Mutated_Character.BP_Mutated_Character_C|SetSwitched%20to%20Metroid%20 _returnvalue false)
  (Variables|Default|SetSwitched%20to%20Mutation true)
  (Transformation|SetActorLocation "-5237.000000,-190.000000,-604.000000" false false)
  (CameraFades|StartCameraFade (Game|GetPlayerCameraManager 0) 1.0 0.0 1.0 "(R=0.000000,G=0.000000,B=0.000000,A=1.000000)" false false)
  (Utilities|FlowControl|Delay 1.0))

(event Custom|Wallslide%20Test
  ;[1 1 1] Damage yeme testi
  (Variables|Wallslide|SetIsWallslide true))

(event Custom|Jump%20Test
  (Variables|Jump|SetisJumping true)
  (if (not (Variables|Wallslide|GetIsWallslide))
    (Character|Jump)
    (Character|Jump)))

(event Custom|ConsistentDamage
  ;[1 0.6234 0.4637] Apply Constant Damage To Player
  (if (Variables|Default|GetSwitched%20to%20Mutation)
    _))

(event Custom|Heal
  ;[1 1 1] Heal
  (bind _output_get (Variables|Health|SetHealth (+ (/ (Variables|Health|GetHealing%20Rate) (Variables|Health|GetHealth)) (Variables|Health|GetHealth)))))

(event Custom|Check%20Falling%20Speed
  ;[0.1672 0.2024 1] Fall Damage
  ;;[1 1 1] Check if player is falling. During falling, keep calculating fall damage.
  (if (not (Variables|Default|GetSwitched%20to%20Mutation))
    (if (not (AI|Components|NavMovement|IsFalling (Variables|Character|GetCharacterMovement)))
      (Game|Damage|ApplyDamage self (Variables|Jump|GetFallDamageAmount) 0 0)
      (Variables|Jump|SetFallDamageAmount 0.0)
      (else
        ;;[1 1 1] These process will be repeated if player is still falling.
        (CallFunction|CalculateFallDamageAmount (Math|Vector|VectorLength (Math|Vector|MakeVector 0.0 0.0 (.z (Transformation|GetVelocity)))))
        (Utilities|FlowControl|Delay 0.1)
        (CallFunction|CheckFallingSpeed)))))

(event Custom|Start%20Dot
  ;[1 1 1] Getting Damaged Over Time
  (bind _returnvalue (Utilities|Time|SetTimerbyEvent (delegate Custom|Dot) (Variables|DamageTimer|GetDuration) true))
  (Variables|DamageTimer|SetDot%20Timer _returnvalue))

(event Custom|Dot
  ;[1 1 1] Getting Damaged Over Time
  (Game|Damage|ApplyDamage self (Variables|Health|GetDamage%20Recieved) 0 0))

(event Custom|End%20Dot
  ;[1 1 1] Getting Damaged Over Time
  (Utilities|Time|ClearandInvalidateTimerbyHandle (Variables|DamageTimer|GetDot%20Timer)))

(event Custom|Stuck%20Y
  (bind _returnvalue (Transformation|GetActorLocation))
  ;[1 1 1] Make sure player has correct y axis
  (if (not (Variables|Default|GetSwitched%20to%20Mutation))
    (if (not (== (.y (Transformation|GetWorldLocation (Variables|Default|GetSprite self))) (Variables|Default|GetAxisPos)))
      (Transformation|SetActorLocation (Math|Vector|MakeVector (.x _returnvalue) -1.9e+02 (.z _returnvalue)) false false))))

(event EventBeginPlay
  (Transformation|SetRelativeScale3D (Variables|Default|GetCapsuleComponent self) "0.800000,0.800000,0.800000")
  (if (not (Variables|Default|GetSwitched%20to%20Mutation))
    (Utilities|FlowControl|Sequence
      (:then_0
        (bind _returnvalue (UserInterface|CreateWidget "/Game/Assets/UI_Assets/Widgets/Healthbar_Widget.Healthbar_Widget_C"))
        (bind _output_get (Variables|General|SetMainWidget _returnvalue))
        (UserInterface|Viewport|AddtoViewport _output_get 0))
      (:then_1
        (bind _returnvalue_2 (UserInterface|CreateWidget "/Game/Assets/Inventory_Assets/UI/Inventory.Inventory_C"))
        (bind _output_get_2 (Variables|Inventory|Setinventory _returnvalue_2))
        (UserInterface|Viewport|AddtoViewport _output_get_2 0)
        (Default|AddtoInventory(MapChange) _output_get_2)
        (Widget|RemovefromParent _output_get_2)))))

(event EventOnMovementModeChanged
  (params (PrevMovementMode :type EMovementMode%20Enum :default "MOVE_None") (NewMovementMode :type EMovementMode%20Enum :default "MOVE_None") (PrevCustomMode :type Byte :default 0) (NewCustomMode :type Byte :default 0))
  ;[0.1672 0.2024 1] Fall Damage
  (if (not (Variables|Default|GetSwitched%20to%20Mutation))
    (if (Utilities|Enum|Equal(Enum) NewMovementMode "MOVE_Falling")
      (Variables|Default|SetFalling%20Start%20Position 0.0)
      ;;[1 1 1] These process will be repeated if player is still falling.
      (CallFunction|CalculateFallDamageAmount (Math|Vector|VectorLength (Math|Vector|MakeVector 0.0 0.0 (.z (Transformation|GetVelocity)))))
      (Utilities|FlowControl|Delay 0.1)
      (CallFunction|CheckFallingSpeed))))

(event EventTick
  (params (DeltaSeconds :type Float%20%28single-precision%29))
  (if (not (Variables|Default|GetSwitched%20to%20Mutation))
    (CallFunction|StuckY)
    ;[1 1 1] animation
    (CallFunction|HandleAnimation)
    (CallFunction|HandleRotation)
    (CallFunction|WallSlide)))

(event Game|Damage|EventAnyDamage
  (params (Damage :type Float%20%28single-precision%29) (DamageType :type Damage%20Type%20Object%20Reference) (InstigatedBy :type Controller%20Object%20Reference) (DamageCauser :type Actor%20Object%20Reference))
  ;[1 1 1] Player Taking Damage
  (bind _output_get (Variables|Health|SetHealth (Math|Float|Clamp(Float) (- (Variables|Health|GetHealth) Damage) 0.0 (Variables|Health|GetDefault%20Health))))
  (bind _returnvalue (Actor|GetActorOfClass "/Game/Blueprints/Chracter_Blueprint/BP_Mutated_Character.BP_Mutated_Character_C"))
  (Variables|Paper2DCharacter_C|SetHealth _returnvalue _output_get)
  (if (and (<= (Variables|Health|GetHealth) 0.0) (not (Variables|Health|GetIs%20Dead)))
    (Variables|Health|SetIs%20Dead true)
    (CallFunction|PlayerDeath)))

(event EventOnLanded
  (params (Hit :type Hit%20Result%20Structure%20%28by%20ref%29))
  ;[1 1 1] Jump landing
  (if (not (Variables|Default|GetSwitched%20to%20Mutation))
    (Variables|Jump|SetjumpCount 0)
    (Variables|Jump|SetisJumping false)))

(event Input|ActionEvents|InputActionJump
  (params (Key :type Key%20Structure :default "None"))
  (:Pressed
    (if (not (Variables|Default|GetSwitched%20to%20Mutation))
      (Variables|Jump|SetisJumping true)
      (if (Variables|Wallslide|GetIsWallslide)
        ;[1 0.6234 0.4637] Wall Jump
        (Character|LaunchCharacter (+ (* (Transformation|GetActorForwardVector) -3e+02) "0,0,600.000000") false false)
        (else
          ;[1 1 1] Jumping
          (Character|Jump)
          (Math|Integer|IncrementInt (Variables|Jump|GetjumpCount)
            (:%20%20
              _))))
      ;[0.32 1 0.9402] Play Jump Sound FX
      (if (<= (Variables|Jump|GetjumpCount) 2)
        (Audio|PlaySoundatLocation "/Game/MusicAndSfx/JumpCue.JumpCue" (Transformation|GetWorldLocation (Variables|Default|GetCapsuleComponent)) "0, 0, 0" 1.0 1.0 0.0 0 0 0 0))))
  (:Released
    (if (not (Variables|Default|GetSwitched%20to%20Mutation))
      (Character|StopJumping))))

(event Input|ActionEvents|InputActionInteractNPC
  (params (Key :type Key%20Structure :default "None")))

(event Input|ActionEvents|InputActionInventory
  (params (Key :type Key%20Structure :default "None"))
  (bind _returnvalue (Game|GetPlayerController 0))
  (bind _inventory (Variables|Inventory|Getinventory))
  ;[1 0.6234 0.4637] show invenory when I is pressed
  (:Pressed
    (if (not (Variables|Default|GetSwitched%20to%20Mutation))
      (Utilities|FlowControl|FlipFlop
        (:A
          (Game|SetGamePaused true)
          (UserInterface|Viewport|AddtoViewport _inventory 0)
          (Variables|/Script/Engine.PlayerController|SetbShowMouseCursor _returnvalue true)
          (Input|SetInputModeGameandUI _returnvalue (Variables|Inventory|Getinventory) "DoNotLock" true))
        (:B
          (Game|SetGamePaused false)
          (Widget|RemovefromParent _inventory)
          (Variables|/Script/Engine.PlayerController|SetbShowMouseCursor _returnvalue false)
          (Input|SetInputModeGameOnly _returnvalue))))))

(event Input|ActionEvents|InputActionFireGun
  (params (Key :type Key%20Structure :default "None"))
  ;[1 0.6234 0.4637] firing bullet every 0.3 seconds when left mouse is pressed
  (:Pressed
    (if (not (Variables|Default|GetSwitched%20to%20Mutation))
      (bind _returnvalue (Utilities|Time|SetTimerbyEvent (delegate Custom|Spawn%20Bullets) (Variables|bullet|GetfireRate) true))
      (Variables|bullet|SetfireBulletEvent _returnvalue)
      (if (Variables|Jump|GetisJumping)
        (Variables|Bullet|SetisShooting false :!label _label)
        (Utilities|Time|ClearandInvalidateTimerbyHandle (Variables|bullet|GetfireBulletEvent))
        (else
          (Variables|Bullet|SetisShooting true)
          ;;[1 1 1] spawns bullet
          (Game|SpawnActorfromClass (Utilities|Array|Get(acopy) (Variables|Bullet|GetbulletTypes) (Variables|bullet|GetselectedBulletIndex)) (Transformation|GetWorldTransform (Variables|Default|GetbulletSpawnPoint)) "Undefined" 0 0)))))
  (:Released
    (goto _label)))

(event Input|AxisEvents|InputAxisMovement
  (params (AxisValue :type Float%20%28single-precision%29))
  ;[1 1 1] Movement
  (if (not (Variables|Default|GetSwitched%20to%20Mutation))
    (Pawn|Input|AddMovementInput "1.000000, 0,0.000000" AxisValue false)
    ;;[1 1 1] Set the Movement Direction According to Axis
    (if (> AxisValue 0.0)
      (Variables|PlayerRotation|SetisMovingRight true)
      (elif (< AxisValue 0.0)
        (Variables|PlayerRotation|SetisMovingRight false)))))

(event Input|KeyboardEvents|M
  (params (Key :type Key%20Structure :default "None"))
  (:Pressed
    (CallFunction|Mutation)))

(event Input|KeyboardEvents|O
  (params (Key :type Key%20Structure :default "None")))

(event Input|KeyboardEvents|8
  (params (Key :type Key%20Structure :default "None"))
  (:Pressed
    (Transformation|SetActorLocation "-847.381775,-190.000000,-3624.127441" false false)))

(event Input|KeyboardEvents|7
  (params (Key :type Key%20Structure :default "None"))
  (:Pressed
    (Transformation|SetActorLocation "1000.000000,-190.000000,-4270.000000" false false)))

(event Input|KeyboardEvents|R
  (params (Key :type Key%20Structure :default "None")))

(event Input|KeyboardEvents|CCedille
  (params (Key :type Key%20Structure :default "None")))

(event Input|KeyboardEvents|Right
  (params (Key :type Key%20Structure :default "None")))

(event Input|KeyboardEvents|0
  (params (Key :type Key%20Structure :default "None"))
  (:Pressed
    (Transformation|SetActorLocation "1390.000000,-190.000000,-7510.000000" false false)))

(event Input|KeyboardEvents|9
  (params (Key :type Key%20Structure :default "None"))
  (:Pressed
    (Transformation|SetActorLocation "2611.343750,-190.000000,-6185.974609" false false)))

(event Input|KeyboardEvents|Escape
  (params (Key :type Key%20Structure :default "None"))
  (bind _returnvalue (Game|GetPlayerController 0))
  ;[1 0.6234 0.4637] show invenory when I is pressed
  (:Pressed
    (if (not (Variables|Default|GetSwitched%20to%20Mutation))
      (Game|SetGamePaused false)
      (Widget|RemovefromParent (Variables|Inventory|Getinventory))
      (Variables|/Script/Engine.PlayerController|SetbShowMouseCursor _returnvalue false)
      (Input|SetInputModeGameOnly _returnvalue))))

(event Input|KeyboardEvents|E
  (params (Key :type Key%20Structure :default "None"))
  ;[0.1672 0.2024 1] Pick Inventory Item Up
  (:Pressed
    (CallFunction|PickInventoryItem)))

(event Input|KeyboardEvents|1
  (params (Key :type Key%20Structure :default "None"))
  ;[0.1672 0.2024 1] change the weapon (will need adjustments)
  (:Pressed
    (Variables|bullet|SetselectedBulletIndex 0)))

(event Input|KeyboardEvents|2
  (params (Key :type Key%20Structure :default "None"))
  ;[0.1672 0.2024 1] change the weapon (will need adjustments)
  (:Pressed
    (if (Variables|Bullet|GetmissileActivated)
      (Variables|bullet|SetselectedBulletIndex 1))))

(event Input|KeyboardEvents|3
  (params (Key :type Key%20Structure :default "None"))
  ;[0.1672 0.2024 1] change the weapon (will need adjustments)
  (:Pressed
    (if (Variables|Bullet|GetlaserActivated)
      (Variables|bullet|SetselectedBulletIndex 2))))

(event Input|KeyboardEvents|7
  (params (Key :type Key%20Structure :default "None"))
  (:Pressed
    (bind _returnvalue (Actor|GetActorOfClass "/Game/Blueprints/Enemy_Bluprints/ProjectileEnemy_BP.ProjectileEnemy_BP_C"))
    (Default|StartShootingPlayer _returnvalue)))

(event Input|KeyboardEvents|8
  (params (Key :type Key%20Structure :default "None"))
  (:Pressed
    (bind _returnvalue (Actor|GetActorOfClass "/Game/Blueprints/Enemy_Bluprints/ProjectileEnemy_BP.ProjectileEnemy_BP_C"))
    (Default|StopShootingPlayer _returnvalue)))

(event Input|KeyboardEvents|H
  (params (Key :type Key%20Structure :default "None"))
  ;[1 1 1] Damage yeme testi
)

(fn ConstructionScript
  (Variables|Health|SetHealth (Variables|Health|GetDefault%20Health)))

(fn PlayerDeath
  (bind _returnvalue (UserInterface|CreateWidget "/Game/Assets/UI_Assets/Widgets/PlayerDeath_Widget.PlayerDeath_Widget_C"))
  (UserInterface|Viewport|AddtoViewport _returnvalue 0)
  (Game|SetGamePaused true)
  (Variables|/Script/Engine.PlayerController|SetbShowMouseCursor (Game|GetPlayerController 0) true))

(fn PlayerTakeDamage
  (params (Enemy :type Actor%20Object%20Reference))
  (bind _asenemy_blueprint (Utilities|Casting|CastToEnemyBlueprint Enemy))
  (Game|Damage|ApplyDamage self (Variables|/Game/Blueprints/Enemy_Bluprints/EnemyBlueprint.EnemyBlueprint_C|GetBase%20Damage _asenemy_blueprint) 0 _asenemy_blueprint))

(fn CalculateFallDamageAmount
  (params (velocity :type Float%20%28double-precision%29))
  (if (not (Variables|Wallslide|GetIsWallslide))
    (if (not (<= velocity 6.5e+02))
      (if (<= velocity 8e+02)
        (Variables|Jump|SetFallDamageAmount 25.0)
        (elif (<= velocity 9e+02)
          (Variables|Jump|SetFallDamageAmount 5e+01)
          (elif (<= velocity 1e+03)
            (Variables|Jump|SetFallDamageAmount 75.0)
            (else
              (Variables|Jump|SetFallDamageAmount 1e+02))))))))

(fn WallSlide
  (bind _returnvalue (Transformation|GetActorLocation))
  ;[0.1672 0.2024 1] Wall Slide Function
  (if (AI|Components|NavMovement|IsFalling (Variables|Character|GetCharacterMovement))
    (bind (_outhit _returnvalue_2) (Collision|LineTraceByChannel _returnvalue (+ _returnvalue (* (Transformation|GetActorForwardVector) 2e+01)) "TraceTypeQuery1" false 0 "None"))
    (if _returnvalue_2
      (Variables|Wallslide|SetIsWallslide true)
      (Transformation|SetActorRotation (Math|Rotator|MakeRotator 0.0 0.0 (+ (.yaw (Math|Conversions|RotationFromXVector (.ImpactNormal (Collision|BreakHitResult _outhit)))) 1.8e+02)))
      (Variables|/Script/Engine.MovementComponent|SetVelocity (Variables|Character|GetCharacterMovement) (Math|Interpolation|VInterptoConstant (Variables|/Script/Engine.MovementComponent|GetVelocity (Variables|Character|GetCharacterMovement)) "0, 0, 0" (Utilities|Time|GetWorldDeltaSeconds) 9e+02))
      (else
        (Variables|Wallslide|SetIsWallslide false :!label _label)))
    (else
      (goto _label))))

(fn PickInventoryItem
  ;[0.1672 0.2024 1] picks up the item when e is pressd
  (bind _array_element (Utilities|Array|ForEachLoopwithBreak (Collision|GetOverlappingActors "/Script/Engine.Actor" :!class /Script/Engine.Actor) :!label _label)
    (:LoopBody
      (if (Utilities|DoesObjectImplementInterface _array_element "/Game/Blueprints/Consumable_Blueprints/Interact.Interact_C")
        (Class|Interact|Interact(Message) _array_element)
        (goto _label Break)))))

(fn HandlePlayerRotaion
  (Math|Float|CompareFloat (.x (Variables|/Script/Engine.MovementComponent|GetVelocity (Variables|Character|GetCharacterMovement))) 0.0
    (:>
      (Pawn|SetControlRotation (Pawn|GetController) (Math|Rotator|MakeRotator 0.0 0.0 0.0) :!label _label))
    (:==
      (if (Variables|PlayerRotation|GetisMovingRight)
        (goto _label)
        (else
          (Pawn|SetControlRotation (Pawn|GetController) (Math|Rotator|MakeRotator 0.0 0.0 1.8e+02) :!label _label_2))))
    (:<
      (goto _label_2))))

(fn ApplyDamagetoPlayer
  (params (damageAmount :type Float%20%28double-precision%29))
  (bind _output_get (Variables|Health|SetHealth (Math|Float|Clamp(Float) (- (Variables|Health|GetHealth) damageAmount) 0.0 (Variables|Health|GetDefault%20Health))))
  (if (<= _output_get 0.0)
    (CallFunction|PlayerDeath)))

(fn ConsistentDamageTimerforTrap
  (params (damageAmount :type Float%20%28double-precision%29) (damageDuration :type Float%20%28double-precision%29) (Handle :type Timer%20Handle%20Structure%20%28by%20ref%29) (time :type Float%20%28double-precision%29) (timerLoopAmount :type Float%20%28double-precision%29))
  (if (< time damageDuration)
    (CallFunction|ApplyDamagetoPlayer damageAmount)
    (Variables|Default|SetcurrentTime (+ (Variables|Default|GetcurrentTime) 0.5))
    (else
      (Utilities|Time|ClearandInvalidateTimerbyHandle Handle)
      ;[1 0.6234 0.4637] reset the timer value and decrease the trap count since the continues damage stops
      (Variables|Default|SetcurrentTime 0.0)
      (if (> (Variables|Default|GetsteppedTrapCount) 0)
        (bind _result (Math|Integer|DecrementInt (Variables|Default|GetsteppedTrapCount))
          (:%20%20
            (Variables|Default|SetsteppedTrapCount _result)))))))

(fn PlayerRef
  (return self))