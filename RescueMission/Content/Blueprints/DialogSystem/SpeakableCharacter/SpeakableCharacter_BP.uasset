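; Speakable 2D NPC that opens a dialog widget when a Paper2D character enters its box and closes it on exit.
; Construction applies its flipbook and scale; overlap also yaws it to the negated player yaw.
; Show and remove functions toggle the widget, cursor and input mode.
; While dialog is open, Tick compares displayed text to the last line, and on "GameEnder"-tagged NPCs pauses the game, plays a sound and shows the ending screen.
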(event OnComponentBeginOverlap(Box)
  (params (OverlappedComponent :type Primitive%20Component%20Object%20Reference) (OtherActor :type Actor%20Object%20Reference) (OtherComp :type Primitive%20Component%20Object%20Reference) (OtherBodyIndex :type Integer) (bFromSweep :type Boolean) (SweepResult :type Hit%20Result%20Structure%20%28by%20ref%29))
  (Utilities|Casting|CastToPaper2DCharacter OtherActor)
  (CallFunction|ShowDialog)
  (Transformation|SetActorRotation (Math|Rotator|MakeRotator 0.0 0.0 (* (.yaw (Transformation|GetActorRotation (Game|GetPlayerCharacter 0))) -1.0))))

(event OnComponentEndOverlap(Box)
  (params (OverlappedComponent :type Primitive%20Component%20Object%20Reference) (OtherActor :type Actor%20Object%20Reference) (OtherComp :type Primitive%20Component%20Object%20Reference) (OtherBodyIndex :type Integer))
  (CallFunction|RemoveDialog))

(event EventTick
  (params (DeltaSeconds :type Float%20%28single-precision%29))
  (bind _dialog (Variables|Default|Getdialog))
  (if (Variables|Default|GetCheckLast)
    (if (and (Utilities|Enum|Equal(Enum) (Utilities|Array|Get(acopy) _dialog (Utilities|Array|LastIndex _dialog)) (Class|TextBlock|GetText (Variables|/Game/Blueprints/DialogSystem/Dialog_Widget.Dialog_Widget_C|GetDialogText (Variables|Default|GetdialogWidget)))) (Actor|ActorHasTag "GameEnder"))
      (Game|SetGamePaused true)
      (Audio|PlaySound2D "/Game/MusicAndSfx/Microsoft_Windows_98_Startup_Sound.Microsoft_Windows_98_Startup_Sound" 1.0 1.0 0.0 0 0)
      (bind _returnvalue (UserInterface|CreateWidget "/Game/Ending_Screen_Widget.Ending_Screen_Widget_C"))
      (UserInterface|Viewport|AddtoViewport _returnvalue 0))))

(fn ConstructionScript
  (Sprite|SetFlipbook (Variables|Default|GetSprite) (Variables|Default|GetNPCSprite))
  (Transformation|SetWorldScale3D (Variables|Default|GetSprite) (Variables|Default|GetScale)))

(fn ShowDialog
  (bind _returnvalue (Game|GetPlayerController 0))
  (if (not (Variables|Default|GetisWidgetOn))
    (Variables|/Script/Engine.PlayerController|SetbShowMouseCursor _returnvalue true)
    (Variables|Default|SetCheckLast true)
    (Input|SetInputModeGameandUI _returnvalue 0 "DoNotLock" true)
    (bind _returnvalue_2 (UserInterface|CreateWidget "/Game/Blueprints/DialogSystem/Dialog_Widget.Dialog_Widget_C" 0 self))
    (bind _output_get (Variables|Default|SetdialogWidget _returnvalue_2))
    (UserInterface|Viewport|AddtoViewport _output_get 0)
    (Variables|Default|SetisWidgetOn true)))

(fn RemoveDialog
  (bind _returnvalue (Game|GetPlayerController 0))
  (if (Variables|Default|GetisWidgetOn)
    (Variables|Default|SetCheckLast false)
    (Widget|RemovefromParent (Variables|Default|GetdialogWidget))
    (Variables|Default|SetisWidgetOn false)
    (Variables|/Script/Engine.PlayerController|SetbShowMouseCursor _returnvalue false)
    (Input|SetInputModeGameOnly _returnvalue)))