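; BP_EnemyBullet is an enemy projectile that damages the player on overlap and expires after a short lifetime.
; BeginPlay passes the player's capsule to ProjectileMovement's SetInterpolatedComponent, beside a Turkish note that player targeting still needs adding.
; Sphere overlap obtains the player through PlayerRefMessage and applies DamageAmount once.
; The hit-flag and quick-destroy branch is disconnected, so the bullet survives hits until its timer ends.
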(event OnComponentBeginOverlap(collisionSphere)
  (params (OverlappedComponent :type Primitive%20Component%20Object%20Reference) (OtherActor :type Actor%20Object%20Reference) (OtherComp :type Primitive%20Component%20Object%20Reference) (OtherBodyIndex :type Integer) (bFromSweep :type Boolean) (SweepResult :type Hit%20Result%20Structure%20%28by%20ref%29))
  (bind _playerref (Class|PlayerInterface|PlayerRef(Message) OtherActor))
  (Utilities|IsValid _playerref
    (:Is%20Valid
      (Utilities|FlowControl|DoOnce false
        (:Completed
          (Game|Damage|ApplyDamage _playerref (Variables|Default|GetdamageAmount) 0 0))))))

(event EventBeginPlay
  (bind _aspaper_2dcharacter (Utilities|Casting|CastToPaper2DCharacter (Game|GetPlayerCharacter 0)))
  ;[1 1 1] Buraya Player'ı Targetleyip Gitme Koymalıyız
  (Game|Components|ProjectileMovement|Interpolation|SetInterpolatedComponent (Variables|Default|GetProjectileMovement) (Variables|/Script/Engine.Character|GetCapsuleComponent _aspaper_2dcharacter))
  (if (not (Variables|Default|GethasHitPlayer))
    (Utilities|FlowControl|Delay 3.0)
    (Actor|DestroyActor)))

(event Collision|EventActorBeginOverlap
  (params (OtherActor :type Actor%20Object%20Reference)))

(event EventTick
  (params (DeltaSeconds :type Float%20%28single-precision%29)))

(fn ConstructionScript)