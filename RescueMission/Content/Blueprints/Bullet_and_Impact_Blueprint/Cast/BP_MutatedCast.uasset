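; BP_MutatedCast is a flipbook spell cast actor that damages a regular enemy or boss it hits.
; A component hit on the Spell flipbook casts to EnemyBlueprint, then BP_Boss, and applies fixed damage, with a DamagedApplied flag limiting it to one target once.
; The actor lives only as long as the animation, destroying itself after the flipbook's length or when playback finishes, not on impact.
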(event OnComponentHit(Spell)
  (params (HitComponent :type Primitive%20Component%20Object%20Reference) (OtherActor :type Actor%20Object%20Reference) (OtherComp :type Primitive%20Component%20Object%20Reference) (NormalImpulse :type Vector :default "0, 0, 0") (Hit :type Hit%20Result%20Structure%20%28by%20ref%29))
  (bind _asenemy_blueprint (Utilities|Casting|CastToEnemyBlueprint OtherActor)
    (:then
      (if (not (Variables|Default|GetDamaged%20Applied))
        (Variables|Default|SetDamaged%20Applied true)
        (Game|Damage|ApplyDamage _asenemy_blueprint 3e+01 0 0)))
    (:CastFailed
      (bind _asbp_boss (Utilities|Casting|CastToBP_Boss OtherActor))
      (if (not (Variables|Default|GetDamaged%20Applied))
        (Variables|Default|SetDamaged%20Applied true)
        (Game|Damage|ApplyDamage _asbp_boss 3e+01 0 0)))))

(event OnFinishedPlaying(Spell)
  (Actor|DestroyActor))

(event OnComponentBeginOverlap(Spell)
  (params (OverlappedComponent :type Primitive%20Component%20Object%20Reference) (OtherActor :type Actor%20Object%20Reference) (OtherComp :type Primitive%20Component%20Object%20Reference) (OtherBodyIndex :type Integer) (bFromSweep :type Boolean) (SweepResult :type Hit%20Result%20Structure%20%28by%20ref%29)))

(event EventBeginPlay
  (Variables|Default|SetDamaged%20Applied false)
  (Utilities|FlowControl|Delay (Class|PaperFlipbookComponent|GetFlipbookLength (Variables|Default|GetSpell)))
  (Actor|DestroyActor))

(event Collision|EventActorBeginOverlap
  (params (OtherActor :type Actor%20Object%20Reference)))

(fn ConstructionScript)