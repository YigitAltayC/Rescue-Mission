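; BringerCast_BP is a short-lived spell cast actor, likely for a Bringer character, shown as a Paper2D flipbook that deals damage on overlap.
; The Spell flipbook component's begin-overlap applies damage to the first Paper2D character it touches, guarded by a flag so it hits only once.
; The actor destroys itself after the flipbook's length, or when the animation finishes playing.
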(event OnFinishedPlaying(Spell)
  (Actor|DestroyActor))

(event OnComponentBeginOverlap(Spell)
  (params (OverlappedComponent :type Primitive%20Component%20Object%20Reference) (OtherActor :type Actor%20Object%20Reference) (OtherComp :type Primitive%20Component%20Object%20Reference) (OtherBodyIndex :type Integer) (bFromSweep :type Boolean) (SweepResult :type Hit%20Result%20Structure%20%28by%20ref%29))
  (bind _aspaper_2dcharacter (Utilities|Casting|CastToPaper2DCharacter OtherActor))
  (if (not (Variables|Default|GetDamaged%20Applied))
    (Variables|Default|SetDamaged%20Applied true)
    (Game|Damage|ApplyDamage _aspaper_2dcharacter 1.0 0 0)))

(event EventBeginPlay
  (Variables|Default|SetDamaged%20Applied false)
  (Utilities|FlowControl|Delay (Class|PaperFlipbookComponent|GetFlipbookLength (Variables|Default|GetSpell)))
  (Actor|DestroyActor))

(event Collision|EventActorBeginOverlap
  (params (OtherActor :type Actor%20Object%20Reference)))

(fn ConstructionScript)