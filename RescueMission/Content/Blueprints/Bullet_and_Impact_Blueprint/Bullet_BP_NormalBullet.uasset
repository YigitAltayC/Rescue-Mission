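; Normal bullet projectile Blueprint that specializes a parent bullet class by supplying its sound, impact and damage settings.
; On BeginPlay it assigns a laser fire sound, sets ImpactClass to self and sets damage, then calls the parent BeginPlay.
; The construction script runs the parent's, then gives the projectile movement component matching initial and maximum speeds.
; Overlap and Tick events are disabled, and no collision logic appears here.
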(event EventBeginPlay
  (Variables|Default|SetFire%20Sound%20FX "/Game/MusicAndSfx/NormalLaserCue.NormalLaserCue")
  (Variables|Default|SetImpact%20Class self)
  (Variables|Default|Setdamage 1e+01)
  (|CallParentFunction))

(event Collision|EventActorBeginOverlap
  (params (OtherActor :type Actor%20Object%20Reference))
  (|CallParentFunction OtherActor) ; This node is disabled and will not be called.\nDrag off pins to build functionality.
)

(event EventTick
  (params (DeltaSeconds :type Float%20%28single-precision%29))
  (|CallParentFunction DeltaSeconds) ; This node is disabled and will not be called.\nDrag off pins to build functionality.
)

(fn ConstructionScript
  (bind _projectilemovement (Variables|Default|GetProjectileMovement))
  (|CallParentFunction)
  (Variables|/Script/Engine.ProjectileMovementComponent|SetInitialSpeed _projectilemovement 5e+02)
  (Variables|/Script/Engine.ProjectileMovementComponent|SetMaxSpeed _projectilemovement 5e+02))