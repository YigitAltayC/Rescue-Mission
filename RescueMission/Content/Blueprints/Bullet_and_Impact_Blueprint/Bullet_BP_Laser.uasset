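; Laser variant of a bullet projectile that damages enemies and bursts on impact.
; BeginPlay sets the blue laser fire and explosion sounds and the damage before calling the parent, and the construction script sets the projectile speed.
; Sphere overlap damages "enemy"-tagged actors, then spawns LaserImpact_BP and destroys the bullet; "Wall"-tagged actors trigger only the impact and destruction.
; The impact class is hardcoded, as the ImpactClass setter is left unconnected.
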(event OnComponentBeginOverlap(Sphere)
  (params (OverlappedComponent :type Primitive%20Component%20Object%20Reference) (OtherActor :type Actor%20Object%20Reference) (OtherComp :type Primitive%20Component%20Object%20Reference) (OtherBodyIndex :type Integer) (bFromSweep :type Boolean) (SweepResult :type Hit%20Result%20Structure%20%28by%20ref%29))
  ;[1 1 1] Hoş ama impactları parentlasak mı ? ya da Impact class diye bir şey yazmıştım BulletBP içine, BeginPlay'de onu setleyip kurtulsak ? Ben yapamadım, biri yapsn
  (if (Actor|ActorHasTag OtherActor "enemy")
    (Variables|Default|SethasHitEnemy true)
    (Game|Damage|ApplyDamage OtherActor (Variables|Default|Getdamage) 0 0)
    (Game|SpawnActorfromClass "/Game/Blueprints/Bullet_and_Impact_Blueprint/Impacts/LaserImpact_BP.LaserImpact_BP_C" (Transformation|GetActorTransform) "Undefined" 0 0 :!label _label)
    (Actor|DestroyActor)
    (elif (Actor|ActorHasTag OtherActor "Wall")
      (goto _label))))

(event EventBeginPlay
  (Variables|Default|SetFire%20Sound%20FX "/Game/MusicAndSfx/BlueLaserCue.BlueLaserCue")
  (Variables|Default|SetExplosion%20Sound%20FX "/Game/MusicAndSfx/BlueLaserExplosionCue.BlueLaserExplosionCue")
  (Variables|Default|Setdamage 5.0)
  (|CallParentFunction))

(event Collision|EventActorBeginOverlap
  (params (OtherActor :type Actor%20Object%20Reference))
  (|CallParentFunction OtherActor) ; This node is disabled and will not be called.\nDrag off pins to build functionality.
)

(event EventTick
  (params (DeltaSeconds :type Float%20%28single-precision%29))
  (|CallParentFunction DeltaSeconds) ; This node is disabled and will not be called.\nDrag off pins to build functionality.
)

(fn ConstructionScript
  (bind _projectilemovement (Variables|Default|GetProjectileMovement))
  (|CallParentFunction)
  (Variables|/Script/Engine.ProjectileMovementComponent|SetInitialSpeed _projectilemovement 1.5e+03)
  (Variables|/Script/Engine.ProjectileMovementComponent|SetMaxSpeed _projectilemovement 1.5e+03))