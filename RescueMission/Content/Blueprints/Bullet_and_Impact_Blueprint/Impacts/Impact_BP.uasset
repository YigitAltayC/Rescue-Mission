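; Impact_BP is a short-lived effect actor that plays a randomly chosen 2D impact animation.
; On BeginPlay it sets its PaperFlipbook component to a random entry from the ImpactFlipbooks array.
; It then waits for that flipbook's length and destroys itself, so each impact cleans up after one playback.
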(event EventBeginPlay
  (Sprite|SetFlipbook (Variables|Default|GetPaperFlipbook) (Utilities|Array|Get(acopy) (Variables|Default|GetImpactFlipbooks) (Math|Random|RandomIntegerinRange 0 (Utilities|Array|LastIndex (Variables|Default|GetImpactFlipbooks)))))
  (Utilities|FlowControl|Delay (Class|PaperFlipbookComponent|GetFlipbookLength (Variables|Default|GetPaperFlipbook)))
  (Actor|DestroyActor))

(event Collision|EventActorBeginOverlap
  (params (OtherActor :type Actor%20Object%20Reference)))

(event EventTick
  (params (DeltaSeconds :type Float%20%28single-precision%29)))

(fn ConstructionScript)