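; Bullet actor for a 2D Paper2D game that damages enemies and bosses and spawns an impact effect on hits.
; On BeginPlay it plays a fire sound, doubles its damage if the player's damage potion is used, and destroys itself after a timeout.
; Sphere overlaps with tagged enemies apply damage; these and tile map hits spawn Impact_BP with an explosion sound and destroy the bullet.
; Destroyable objects only spawn the impact, leaving the bullet alive.
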(event OnComponentBeginOverlap(Sphere)
  (params (OverlappedComponent :type Primitive%20Component%20Object%20Reference) (OtherActor :type Actor%20Object%20Reference) (OtherComp :type Primitive%20Component%20Object%20Reference) (OtherBodyIndex :type Integer) (bFromSweep :type Boolean) (SweepResult :type Hit%20Result%20Structure%20%28by%20ref%29))
  ;[1 1 1] Deal Damage When Hıts Enemy / Explode When Hıts Enemy or Walls
  (if (or (Actor|ActorHasTag OtherActor "enemy") (Actor|ActorHasTag OtherActor "Boss"))
    (Variables|Default|SethasHitEnemy true)
    (Game|Damage|ApplyDamage OtherActor (Variables|Default|Getdamage) 0 0)
    (bind _returnvalue (Game|SpawnActorfromClass "/Game/Blueprints/Bullet_and_Impact_Blueprint/Impacts/Impact_BP.Impact_BP_C" (Transformation|GetActorTransform) "Undefined" 0 0 :!label _label))
    (Audio|PlaySoundatLocation (Variables|Default|GetExplosion%20Sound%20FX) (Transformation|GetActorLocation _returnvalue) "0, 0, 0" 1.0 1.0 0.0 0 0 0 0)
    (Actor|DestroyActor)
    (elif (Actor|ActorHasTag OtherActor "DestroyableObject")
      (Game|SpawnActorfromClass "/Game/Blueprints/Bullet_and_Impact_Blueprint/Impacts/Impact_BP.Impact_BP_C" (Transformation|GetActorTransform) "Undefined" 0 0)
      (elif (== (Utilities|GetClass OtherActor) "/Script/Paper2D.PaperTileMapActor")
        (goto _label)))))

(event EventBeginPlay
  (Audio|PlaySoundatLocation (Variables|Default|GetFire%20Sound%20FX) (Transformation|GetActorLocation) "0, 0, 0" 1.0 1.0 0.0 0 0 0 0)
  (bind _aspaper_2dcharacter (Utilities|Casting|CastToPaper2DCharacter (Game|GetPlayerCharacter 0)))
  (if (Variables|/Game/Blueprints/Chracter_Blueprint/Paper2DCharacter.Paper2DCharacter_C|GetisDamagePotionUsed _aspaper_2dcharacter)
    (Variables|Default|Setdamage (* (Variables|Default|Getdamage) 2.0)))
  (if (not (Variables|Default|GethasHitEnemy))
    (Utilities|FlowControl|Delay 3.0)
    (Actor|DestroyActor)))

(fn ConstructionScript)