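; BP_DamageIncreaser is an inventory consumable that gives the player a temporary damage potion effect.
; UseItem sets the IsDamagePotionUsed flag on the player's Paper2DCharacter.
; GoInitialState waits 30 seconds, clears the flag and removes the supplied widget from the WrapBox in the character's main widget.
; The item only toggles the flag and contains no damage calculation.
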(event EventBeginPlay
  (|CallParentFunction))

(event Collision|EventActorBeginOverlap
  (params (OtherActor :type Actor%20Object%20Reference)))

(event EventTick
  (params (DeltaSeconds :type Float%20%28single-precision%29))
  (|CallParentFunction DeltaSeconds) ; This node is disabled and will not be called.\nDrag off pins to build functionality.
)

(event EventUseItem
  (bind _aspaper_2dcharacter (Utilities|Casting|CastToPaper2DCharacter (Game|GetPlayerCharacter 0)))
  (Variables|/Game/Blueprints/Chracter_Blueprint/Paper2DCharacter.Paper2DCharacter_C|SetisDamagePotionUsed _aspaper_2dcharacter true))

(event EventGoInitialState
  (params (widget :type Potion%20Widgets%20Object%20Reference))
  (bind _aspaper_2dcharacter (Utilities|Casting|CastToPaper2DCharacter (Game|GetPlayerCharacter 0)))
  (Utilities|FlowControl|Delay 3e+01)
  (Variables|/Game/Blueprints/Chracter_Blueprint/Paper2DCharacter.Paper2DCharacter_C|SetisDamagePotionUsed _aspaper_2dcharacter false)
  (Class|PanelWidget|RemoveChild (Variables|/Game/Assets/UI_Assets/Widgets/Healthbar_Widget.Healthbar_Widget_C|GetWrapBox (Variables|/Game/Blueprints/Chracter_Blueprint/Paper2DCharacter.Paper2DCharacter_C|GetMainWidget _aspaper_2dcharacter)) widget))

(fn ConstructionScript
  (|CallParentFunction))