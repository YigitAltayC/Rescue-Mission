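; BP_HealthPotion is a health potion inventory item that heals the player when used.
; UseItem adds HealAmount to the Health of player 0's Paper2DCharacter, capped at DefaultHealth.
; GoInitialState removes the supplied widget from the WrapBox in that character's MainWidget.
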(event EventBeginPlay
  (|CallParentFunction))

(event Collision|EventActorBeginOverlap
  (params (OtherActor :type Actor%20Object%20Reference)))

(event EventUseItem
  (bind _aspaper_2dcharacter (Utilities|Casting|CastToPaper2DCharacter (Game|GetPlayerCharacter 0)))
  ;[1 1 1] When Player Uses Health Potion
  (if (>= (+ (Variables|Default|GetHeal%20Amount) (Variables|/Game/Blueprints/Chracter_Blueprint/Paper2DCharacter.Paper2DCharacter_C|GetHealth _aspaper_2dcharacter)) (Variables|/Game/Blueprints/Chracter_Blueprint/Paper2DCharacter.Paper2DCharacter_C|GetDefault%20Health _aspaper_2dcharacter))
    (Variables|/Game/Blueprints/Chracter_Blueprint/Paper2DCharacter.Paper2DCharacter_C|SetHealth _aspaper_2dcharacter (Variables|/Game/Blueprints/Chracter_Blueprint/Paper2DCharacter.Paper2DCharacter_C|GetDefault%20Health _aspaper_2dcharacter))
    (else
      (Variables|/Game/Blueprints/Chracter_Blueprint/Paper2DCharacter.Paper2DCharacter_C|SetHealth _aspaper_2dcharacter (+ (Variables|Default|GetHeal%20Amount) (Variables|/Game/Blueprints/Chracter_Blueprint/Paper2DCharacter.Paper2DCharacter_C|GetHealth _aspaper_2dcharacter))))))

(event EventTick
  (params (DeltaSeconds :type Float%20%28single-precision%29))
  (|CallParentFunction DeltaSeconds) ; This node is disabled and will not be called.\nDrag off pins to build functionality.
)

(event EventGoInitialState
  (params (widget :type Potion%20Widgets%20Object%20Reference))
  (bind _aspaper_2dcharacter (Utilities|Casting|CastToPaper2DCharacter (Game|GetPlayerCharacter 0)))
  (Class|PanelWidget|RemoveChild (Variables|/Game/Assets/UI_Assets/Widgets/Healthbar_Widget.Healthbar_Widget_C|GetWrapBox (Variables|/Game/Blueprints/Chracter_Blueprint/Paper2DCharacter.Paper2DCharacter_C|GetMainWidget _aspaper_2dcharacter)) widget))

(fn ConstructionScript
  (|CallParentFunction))