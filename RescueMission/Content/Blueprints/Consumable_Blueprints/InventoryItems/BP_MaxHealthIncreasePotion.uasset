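; Inventory consumable potion that temporarily boosts the player character's maximum health.
; UseItem multiplies both DefaultHealth and current Health by 1.5.
; A separate GoInitialState event waits four seconds, resets max health to a hardcoded 100, clamps current health to it, and removes the passed widget from the main widget's WrapBox.
; Disconnected leftover nodes hold an earlier version that restores a saved old maximum instead.
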(event EventBeginPlay
  (|CallParentFunction))

(event Collision|EventActorBeginOverlap
  (params (OtherActor :type Actor%20Object%20Reference)))

(event EventTick
  (params (DeltaSeconds :type Float%20%28single-precision%29))
  (|CallParentFunction DeltaSeconds) ; This node is disabled and will not be called.\nDrag off pins to build functionality.
)

(event EventUseItem
  (bind _aspaper_2dcharacter (Utilities|Casting|CastToPaper2DCharacter (Game|GetPlayerCharacter 0)))
  (Variables|/Game/Blueprints/Chracter_Blueprint/Paper2DCharacter.Paper2DCharacter_C|SetDefault%20Health _aspaper_2dcharacter (* (Variables|/Game/Blueprints/Chracter_Blueprint/Paper2DCharacter.Paper2DCharacter_C|GetDefault%20Health _aspaper_2dcharacter) 1.5))
  (Variables|/Game/Blueprints/Chracter_Blueprint/Paper2DCharacter.Paper2DCharacter_C|SetHealth _aspaper_2dcharacter (* (Variables|/Game/Blueprints/Chracter_Blueprint/Paper2DCharacter.Paper2DCharacter_C|GetHealth _aspaper_2dcharacter) 1.5)))

(event EventGoInitialState
  (params (widget :type Potion%20Widgets%20Object%20Reference))
  (bind _aspaper_2dcharacter (Utilities|Casting|CastToPaper2DCharacter (Game|GetPlayerCharacter 0)))
  (Utilities|FlowControl|Delay 4.0)
  (Variables|/Game/Blueprints/Chracter_Blueprint/Paper2DCharacter.Paper2DCharacter_C|SetDefault%20Health _aspaper_2dcharacter 1e+02)
  (if (>= (Variables|/Game/Blueprints/Chracter_Blueprint/Paper2DCharacter.Paper2DCharacter_C|GetHealth _aspaper_2dcharacter) 1e+02)
    (Variables|/Game/Blueprints/Chracter_Blueprint/Paper2DCharacter.Paper2DCharacter_C|SetHealth _aspaper_2dcharacter 1e+02)
    (else
      (Variables|/Game/Blueprints/Chracter_Blueprint/Paper2DCharacter.Paper2DCharacter_C|SetHealth _aspaper_2dcharacter (Variables|/Game/Blueprints/Chracter_Blueprint/Paper2DCharacter.Paper2DCharacter_C|GetHealth _aspaper_2dcharacter))))
  (Class|PanelWidget|RemoveChild (Variables|/Game/Assets/UI_Assets/Widgets/Healthbar_Widget.Healthbar_Widget_C|GetWrapBox (Variables|/Game/Blueprints/Chracter_Blueprint/Paper2DCharacter.Paper2DCharacter_C|GetMainWidget _aspaper_2dcharacter)) widget))

(fn ConstructionScript
  (|CallParentFunction))