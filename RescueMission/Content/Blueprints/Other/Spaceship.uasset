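; Spaceship actor that patrols vertically back and forth between a lower and an upper patrol point.
; BeginPlay detaches both point components so they stay fixed in the world, then picks the first target through a FlipFlop.
; Tick applies a small Z-only offset toward the target, not scaled by delta time, and switches targets when the full 3D distance drops below a small threshold.
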(event Custom|SetPatrolPoint
  ;[1 1 1] Setting points to patrol between
  (Utilities|FlowControl|FlipFlop
    (:A
      (Variables|Default|SetTarget%20Loc (Transformation|GetWorldLocation (Variables|Default|GetDown%20Patrol%20Point))))
    (:B
      (Variables|Default|SetTarget%20Loc (Transformation|GetWorldLocation (Variables|Default|GetUp%20Patrol%20Point))))))

(event EventTick
  (params (DeltaSeconds :type Float%20%28single-precision%29))
  (bind _returnvalue (Transformation|GetActorLocation))
  (bind _target_loc (Variables|Default|GetTarget%20Loc))
  (Transformation|AddWorldOffset (Variables|Default|GetDefaultSceneRoot) (Math|Vector|MakeVector 0.0 0.0 (/ (.z (Math|Vector|GetUnitDirection(Vector) _returnvalue _target_loc)) 3.0)) false false)
  (if (< (Math|Vector|Distance(Vector) _returnvalue _target_loc) 1.0)
    (CallFunction|SetPatrolPoint)))

(event Collision|EventActorBeginOverlap
  (params (OtherActor :type Actor%20Object%20Reference)))

(event EventBeginPlay
  (Transformation|DetachFromComponent (Variables|Default|GetDown%20Patrol%20Point) "KeepWorld" "KeepWorld" "KeepWorld" true)
  (CallFunction|SetPatrolPoint))

(fn ConstructionScript)