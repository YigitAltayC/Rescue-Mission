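; Boss-area gate that raises its cube when the player enters its box trigger and lowers it on exit.
; At BeginPlay it binds to the BossDied events of the first BP_GolemBoss and BP_Demon found, setting a flag after a BossId check.
; Gates marked IsEndGate move only once that flag is set, otherwise printing a debug message.
; Separate open and close timelines lerp the cube between its start and raised positions.
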(event OnComponentBeginOverlap(Box)
  (params (OverlappedComponent :type Primitive%20Component%20Object%20Reference) (OtherActor :type Actor%20Object%20Reference) (OtherComp :type Primitive%20Component%20Object%20Reference) (OtherBodyIndex :type Integer) (bFromSweep :type Boolean) (SweepResult :type Hit%20Result%20Structure%20%28by%20ref%29))
  (if (== OtherActor (Game|GetPlayerCharacter 0))
    (if (Variables|Default|GetIsEndGate)
      (if (Variables|Default|GetBoss%20Died)
        (CallFunction|OpenGate)
        (else
          (Development|PrintString "boss not died")))
      (else
        (CallFunction|OpenGate)))))

(event OnComponentEndOverlap(Box)
  (params (OverlappedComponent :type Primitive%20Component%20Object%20Reference) (OtherActor :type Actor%20Object%20Reference) (OtherComp :type Primitive%20Component%20Object%20Reference) (OtherBodyIndex :type Integer))
  (if (== OtherActor (Game|GetPlayerCharacter 0))
    (if (Variables|Default|GetIsEndGate)
      (if (Variables|Default|GetBoss%20Died)
        (CallFunction|CloseGate)
        (else
          (Development|PrintString "boss not died")))
      (else
        (CallFunction|CloseGate)))))

(event Custom|Close%20Gate
  (bind _newtrack_0 (Timeline|Timeline_1 PlayFromStart)
    (:Update
      (Transformation|SetWorldLocation (Variables|Default|GetCube) (Math|Vector|Lerp(Vector) (Variables|Default|GetEndLoc) (Variables|Default|GetStartLoc) _newtrack_0) false false))))

(event Custom|Open%20Gate
  (bind _newtrack_0 (Timeline|Timeline_0 PlayFromStart)
    (:Update
      (Transformation|SetWorldLocation (Variables|Default|GetCube) (Math|Vector|Lerp(Vector) (Variables|Default|GetStartLoc) (Variables|Default|GetEndLoc) _newtrack_0) false false))))

(event Custom|Boss%20Died_Event_0
  (params (Boss%20Id :type Integer))
  (if (== (Variables|Default|GetBoss%20Id) Boss%20Id)
    (Variables|Default|SetBoss%20Died true)))

(event Custom|CustomEvent
  (params (Boss%20Id :type Integer))
  (if (== (Variables|Default|GetBoss%20Id) Boss%20Id)
    (Variables|Default|SetBoss%20Died true)))

(event EventBeginPlay
  (bind _cube (Variables|Default|GetCube))
  (bind _returnvalue (Transformation|GetWorldLocation _cube))
  (Variables|Default|SetStartLoc _returnvalue)
  (Variables|Default|SetEndLoc (+ _returnvalue "0,0,100.000000"))
  (bind _returnvalue_2 (Actor|GetActorOfClass "/Game/Blueprints/Enemy_Bluprints/Bosses/GolemBoss/BP_GolemBoss.BP_GolemBoss_C"))
  (EventDispatchers|AssignBossDied _returnvalue_2 (delegate Custom|Boss%20Died_Event_0))
  (bind _returnvalue_3 (Actor|GetActorOfClass "/Game/Blueprints/Enemy_Bluprints/Bosses/DemonBoss/BP_Demon.BP_Demon_C"))
  (EventDispatchers|AssignBossDied _returnvalue_3 (delegate Custom|CustomEvent)))

(fn ConstructionScript)