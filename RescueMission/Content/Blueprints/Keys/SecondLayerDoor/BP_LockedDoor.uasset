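; Locked door actor that swings open 90 degrees once the player has every required key.
; When the player enters the trigger box, it shows a key widget and checks every flag in IsDoorKeysPicked.
; If all are set, it waits briefly, removes the widget and runs a timeline that lerps the pivot's rotation.
; Otherwise it resets the check for the next overlap, and leaving the box removes the widget.
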(event OnComponentBeginOverlap(Box)
  (params (OverlappedComponent :type Primitive%20Component%20Object%20Reference) (OtherActor :type Actor%20Object%20Reference) (OtherComp :type Primitive%20Component%20Object%20Reference) (OtherBodyIndex :type Integer) (bFromSweep :type Boolean) (SweepResult :type Hit%20Result%20Structure%20%28by%20ref%29))
  (if (== OtherActor (Game|GetPlayerCharacter 0))
    (if (Variables|Default|GetIsWidgetOn)
      _
      (else
        (bind _returnvalue (UserInterface|CreateWidget "/Game/Assets/UI_Assets/Widgets/DoorKey_Widget.DoorKey_Widget_C"))
        (bind _output_get (Variables|Default|SetDoor%20Widget _returnvalue))
        (UserInterface|Viewport|AddtoViewport _output_get 0)
        (Variables|Default|SetIsWidgetOn true)))
    (for _array_element (Variables|Default|GetIsDoorKeysPicked)
      (if (not _array_element)
        (Variables|Components|SetAreAllKeysPicked false)))
    (if (Variables|Components|GetAreAllKeysPicked)
      (Utilities|FlowControl|Delay 1.0)
      (Widget|RemovefromParent (Variables|Default|GetDoor%20Widget))
      (bind _door_track (Timeline|Door%20Timeline Play)
        (:Update
          (Transformation|SetWorldRotation (Variables|Default|GetDoor%20Pivot) (Math|Rotator|Lerp(Rotator) (Variables|Default|GetStartRotation) (Variables|Default|GetEndRotation) _door_track) false false)))
      (else
        (Variables|Components|SetAreAllKeysPicked true)))))

(event OnComponentEndOverlap(Box)
  (params (OverlappedComponent :type Primitive%20Component%20Object%20Reference) (OtherActor :type Actor%20Object%20Reference) (OtherComp :type Primitive%20Component%20Object%20Reference) (OtherBodyIndex :type Integer))
  (if (== OtherActor (Game|GetPlayerCharacter 0))
    (if (Variables|Default|GetIsWidgetOn)
      (Widget|RemovefromParent (Variables|Default|GetDoor%20Widget))
      (Variables|Default|SetIsWidgetOn false))))

(event EventBeginPlay
  (bind _output_get (Variables|Default|SetStartRotation (Transformation|GetWorldRotation (Variables|Default|GetDoor%20Pivot))))
  (Variables|Default|SetEndRotation (Math|Rotator|MakeRotator (.roll _output_get) (.pitch _output_get) (- (.yaw _output_get) 9e+01))))

(event Collision|EventActorBeginOverlap
  (params (OtherActor :type Actor%20Object%20Reference)))

(event EventTick
  (params (DeltaSeconds :type Float%20%28single-precision%29)))

(fn ConstructionScript)