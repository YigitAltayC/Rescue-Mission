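; Collectible key for the second-layer door: when the player overlaps its box, it marks its KeyIdentifier as picked on the level's BP_LockedDoor and destroys itself.
; Pickups persist in the "keysave2" save slot through SaveGame_BP's DoorKeys array.
; On BeginPlay it loads or creates that save, copies the array to the door, and destroys already-collected BP_SecondLayerKey1 and BP_SecondLayerKey2 actors by hard-coded index.
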(event OnComponentBeginOverlap(Box)
  (params (OverlappedComponent :type Primitive%20Component%20Object%20Reference) (OtherActor :type Actor%20Object%20Reference) (OtherComp :type Primitive%20Component%20Object%20Reference) (OtherBodyIndex :type Integer) (bFromSweep :type Boolean) (SweepResult :type Hit%20Result%20Structure%20%28by%20ref%29))
  (bind _save_game (Variables|Default|GetSave%20Game))
  (if (== OtherActor (Game|GetPlayerCharacter 0))
    (Utilities|Array|SetArrayElem (Variables|/Game/Blueprints/Keys/SecondLayerDoor/BP_LockedDoor.BP_LockedDoor_C|GetIsDoorKeysPicked (Variables|Default|GetDoor%20Ref)) (Variables|Default|GetKeyIdentifier) true)
    (Utilities|Array|SetArrayElem (Variables|/Game/Blueprints/Chracter_Blueprint/SaveGame_BP.SaveGame_BP_C|GetDoorKeys _save_game) (Variables|Default|GetKeyIdentifier) true)
    (SaveGame|SaveGametoSlot _save_game "keysave2")
    (Actor|DestroyActor)))

(event EventBeginPlay
  (bind _returnvalue (Actor|GetActorOfClass "/Game/Blueprints/Keys/SecondLayerDoor/BP_LockedDoor.BP_LockedDoor_C"))
  (Variables|Default|SetDoor%20Ref _returnvalue)
  (CallFunction|Save))

(event Collision|EventActorBeginOverlap
  (params (OtherActor :type Actor%20Object%20Reference)))

(event EventTick
  (params (DeltaSeconds :type Float%20%28single-precision%29)))

(fn ConstructionScript)

(fn Save
  (bind _returnvalue (SaveGame|DoesSaveGameExist "keysave2"))
  (if _returnvalue
    (bind _returnvalue_2 (SaveGame|LoadGamefromSlot "keysave2"))
    (bind _assave_game_bp (Utilities|Casting|CastToSaveGame_BP _returnvalue_2))
    (bind _output_get (Variables|Default|SetSave%20Game _assave_game_bp))
    (Variables|/Game/Blueprints/Keys/SecondLayerDoor/BP_LockedDoor.BP_LockedDoor_C|SetIsDoorKeysPicked (Variables|Default|GetDoor%20Ref) (Variables|/Game/Blueprints/Chracter_Blueprint/SaveGame_BP.SaveGame_BP_C|GetDoorKeys _output_get))
    (for (_array_element _array_index) (Variables|/Game/Blueprints/Chracter_Blueprint/SaveGame_BP.SaveGame_BP_C|GetDoorKeys _output_get)
      (if _array_element
        (switch int _array_index
          (:0
            (bind _returnvalue_3 (Actor|GetActorOfClass "/Game/Blueprints/Keys/SecondLayerDoor/BP_SecondLayerKey1.BP_SecondLayerKey1_C"))
            (Utilities|IsValid _returnvalue_3
              (:Is%20Valid
                (Actor|DestroyActor _returnvalue_3))))
          (:1
            (bind _returnvalue_4 (Actor|GetActorOfClass "/Game/Blueprints/Keys/SecondLayerDoor/BP_SecondLayerKey2.BP_SecondLayerKey2_C"))
            (Utilities|IsValid _returnvalue_4
              (:Is%20Valid
                (Actor|DestroyActor _returnvalue_4)))))))
    (else
      (bind _returnvalue_5 (SaveGame|CreateSaveGameObject "/Game/Blueprints/Chracter_Blueprint/SaveGame_BP.SaveGame_BP_C"))
      (bind _output_get_2 (Variables|Default|SetSave%20Game _returnvalue_5))
      (Variables|/Game/Blueprints/Keys/SecondLayerDoor/BP_LockedDoor.BP_LockedDoor_C|SetIsDoorKeysPicked (Variables|Default|GetDoor%20Ref) (Variables|/Game/Blueprints/Chracter_Blueprint/SaveGame_BP.SaveGame_BP_C|GetDoorKeys _output_get_2))
      (SaveGame|SaveGametoSlot (Variables|Default|GetSave%20Game) "keysave2"))))