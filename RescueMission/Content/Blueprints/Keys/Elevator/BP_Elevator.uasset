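; Key-gated elevator that carries a Paper2D character between its BeginPlay position and ElevatorEndPos.
; Stepping into the Box shows ElevatorKey_Widget and checks every IsElevatorKeysPicked flag; stepping out removes the widget.
; With all keys picked, it hides the widget, waits briefly, then a timeline lerps the root toward the end or back to the start, based on its current position.
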(event OnComponentBeginOverlap(Box)
  (params (OverlappedComponent :type Primitive%20Component%20Object%20Reference) (OtherActor :type Actor%20Object%20Reference) (OtherComp :type Primitive%20Component%20Object%20Reference) (OtherBodyIndex :type Integer) (bFromSweep :type Boolean) (SweepResult :type Hit%20Result%20Structure%20%28by%20ref%29))
  (Utilities|Casting|CastToPaper2DCharacter OtherActor)
  (if (Variables|Default|GetisElevatorWidgetOn)
    _
    (else
      (bind _returnvalue (UserInterface|CreateWidget "/Game/Assets/UI_Assets/Widgets/ElevatorKey_Widget.ElevatorKey_Widget_C"))
      (Variables|Default|Setwidget _returnvalue)
      (UserInterface|Viewport|AddtoViewport _returnvalue 0)
      (Variables|Default|SetisElevatorWidgetOn true)))
  (for _array_element (Variables|Default|GetIsElevatorKeysPicked)
    (if (not _array_element)
      (Variables|Default|SetAreAllKeysPicked false)))
  (Default|ElevatorStepped (Variables|Default|Getwidget))
  (if (Variables|Default|GetAreAllKeysPicked)
    (Widget|RemovefromParent (Variables|Default|Getwidget))
    (if (Utilities|Operators|EqualEqual (Transformation|GetActorLocation) (Variables|Default|GetelevatorStartPos) 1.0)
      ;[1 1 1] moves the elevator down
      (Utilities|FlowControl|Delay 1.0)
      (bind _newtrack_0 (Timeline|Timeline_0 PlayFromStart)
        (:Update
          (Transformation|SetWorldLocation (Variables|Default|GetDefaultSceneRoot) (Math|Vector|Lerp(Vector) (Variables|Default|GetelevatorStartPos) (Variables|Default|GetelevatorEndPos) _newtrack_0) false false)))
      (else
        (Utilities|FlowControl|Delay 1.0)
        (bind _newtrack_0_2 (Timeline|Timeline_1 PlayFromStart)
          (:Update
            (Transformation|SetWorldLocation (Variables|Default|GetDefaultSceneRoot) (Math|Vector|Lerp(Vector) (Variables|Default|GetelevatorEndPos) (Variables|Default|GetelevatorStartPos) _newtrack_0_2) false false)))))
    (else
      (Variables|Default|SetAreAllKeysPicked true))))

(event OnComponentEndOverlap(Box)
  (params (OverlappedComponent :type Primitive%20Component%20Object%20Reference) (OtherActor :type Actor%20Object%20Reference) (OtherComp :type Primitive%20Component%20Object%20Reference) (OtherBodyIndex :type Integer))
  (Utilities|Casting|CastToPaper2DCharacter OtherActor)
  (if (Variables|Default|GetisElevatorWidgetOn)
    (Widget|RemovefromParent (Variables|Default|Getwidget))
    (Variables|Default|SetisElevatorWidgetOn false)))

(event EventBeginPlay
  (Variables|Default|SetelevatorStartPos (Transformation|GetWorldLocation (Variables|Default|GetDefaultSceneRoot))))

(event Collision|EventActorBeginOverlap
  (params (OtherActor :type Actor%20Object%20Reference)))

(event EventTick
  (params (DeltaSeconds :type Float%20%28single-precision%29)))

(fn ConstructionScript)