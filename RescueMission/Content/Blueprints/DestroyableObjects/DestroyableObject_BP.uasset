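; Base Paper2D Blueprint for objects that bullets can break, with child classes supplying the sprites.
; Box overlaps with "Bullet"-tagged actors destroy the bullet and count impacts up to a maximum; the following hit breaks the object.
; Breaking disables collision, swaps to the broken sprite, plays a one-shot flipbook and optionally spawns an actor at an offset.
; When the animation finishes, only the flipbook component is destroyed.
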(event OnComponentBeginOverlap(Box)
  (params (OverlappedComponent :type Primitive%20Component%20Object%20Reference) (OtherActor :type Actor%20Object%20Reference) (OtherComp :type Primitive%20Component%20Object%20Reference) (OtherBodyIndex :type Integer) (bFromSweep :type Boolean) (SweepResult :type Hit%20Result%20Structure%20%28by%20ref%29))
  (bind _impactnumber (Variables|Default|GetimpactNumber))
  (bind _flipbookanimation (Variables|Default|GetflipbookAnimation))
  ;[1 0.6234 0.4637] if the overlaped actor is bullet the impact number is increased
  (if (Actor|ActorHasTag OtherActor "Bullet")
    (Actor|DestroyActor OtherActor)
    (if (< _impactnumber (Variables|Default|GetmaxImpactNumber))
      (Math|Float|IncrementFloat _impactnumber)
      (else
        ;[1 0.6234 0.4637] when the impact number reached the given number the animation will play and the sprite will be changed to the broken item
        (if (== (Variables|Default|GetimpactNumber) (Variables|Default|GetmaxImpactNumber))
          (Collision|SetCollisionEnabled (Variables|Default|GetBox) "NoCollision")
          (Rendering|Components|Sprite|SetSprite (Variables|Default|GetPaperSprite) (Variables|Default|GetnewSprite))
          (Components|Timeline|SetLooping _flipbookanimation false)
          (Sprite|SetFlipbook _flipbookanimation (Variables|Default|Getanimation))
          (Audio|Components|Audio|Play _flipbookanimation)
          (if (Variables|Default|GetshouldSpawnObject)
            (Game|SpawnActorfromClass (Variables|Default|GetActorToSpawn) (Math|Transform|MakeTransform (+ (Transformation|GetActorLocation) (Variables|Default|GetSpawn%20Transform%20Location%20Addition)) "0, 0, 0" (Variables|Default|GetSpawn%20Transform%20Scale)) "AlwaysSpawn" 0 0)))))))

(event OnFinishedPlaying(flipbookAnimation)
  ;[1 0.6234 0.4637] when animation is finished it will be destroyed
  (Components|DestroyComponent (Variables|Default|GetflipbookAnimation)))

(event EventBeginPlay
  ;[1 0.6234 0.4637] sprite will be changed from the child classes
  (Rendering|Components|Sprite|SetSprite (Variables|Default|GetPaperSprite) (Variables|Default|GetnormalSprite)))

(fn ConstructionScript
  (Rendering|Components|Sprite|SetSprite (Variables|Default|GetPaperSprite) (Variables|Default|GetnormalSprite)))