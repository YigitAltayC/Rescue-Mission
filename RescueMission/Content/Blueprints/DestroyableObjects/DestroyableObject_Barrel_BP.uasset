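; Barrel variant of a destroyable object, a child Blueprint that supplies barrel-specific art and durability to its parent class.
; The construction script assigns the normal sprite, a second replacement sprite, the barrel flipbook animation and the maximum impact count, then runs the parent construction script.
; BeginPlay only calls the parent, so all destruction behavior is left to inherited logic.
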(event EventBeginPlay
  (|CallParentFunction))

(event Collision|EventActorBeginOverlap
  (params (OtherActor :type Actor%20Object%20Reference))
  (|CallParentFunction OtherActor) ; This node is disabled and will not be called.\nDrag off pins to build functionality.
)

(event EventTick
  (params (DeltaSeconds :type Float%20%28single-precision%29))
  (|CallParentFunction DeltaSeconds) ; This node is disabled and will not be called.\nDrag off pins to build functionality.
)

(fn ConstructionScript
  (Variables|Default|SetnewSprite "/Game/Assets/DestroyableObject/Destructible_Objects_Sprite_Sheet__1__Sprite_13.Destructible_Objects_Sprite_Sheet__1__Sprite_13")
  (Variables|Default|SetnormalSprite "/Game/Assets/DestroyableObject/Destructible_Objects_Sprite_Sheet__1__Sprite_0.Destructible_Objects_Sprite_Sheet__1__Sprite_0")
  (Variables|Default|Setanimation "/Game/Assets/DestroyableObject/DestroyableBarrelFlipbook.DestroyableBarrelFlipbook")
  (Variables|Default|SetmaxImpactNumber 6.0)
  (|CallParentFunction))