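; BP_EnemyMoveTest is a functional test that checks that a crab enemy moves to its patrol target.
; Each Tick copies the camera's world Y into the Character's AxisPos, then casts Enemy to CrabBlueprint_BP.
; The test succeeds once the enemy is within a small tolerance of the crab's TargetLoc.
; Prepare and start events are empty, no failure branch exists, and the counter logic is unconnected.
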(event EventPrepareTest)

(event EventStartTest)

(event EventTick
  (params (DeltaSeconds :type Float%20%28single-precision%29))
  (bind _enemy (Variables|Default|GetEnemy))
  (Variables|/Game/Blueprints/Chracter_Blueprint/Paper2DCharacter.Paper2DCharacter_C|SetAxisPos (Variables|Default|GetCharacter) (.y (Transformation|GetWorldLocation (Variables|/Script/Engine.CameraActor|GetCameraComponent (Variables|Default|GetCamera)))))
  (bind _ascrab_blueprint (Utilities|Casting|CastToCrabBlueprint_BP _enemy))
  (if (Utilities|Operators|EqualEqual (Transformation|GetActorLocation _enemy) (Variables|/Game/Blueprints/Enemy_Bluprints/CrabBlueprint_BP.CrabBlueprint_BP_C|GetTargetLoc _ascrab_blueprint) 5.0)
    (Class|FunctionalTest|FinishTest "Succeeded" "Enemy Succesfully Patrolled between Points")))

(fn ConstructionScript)