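; BP_CharacterDoubleJumpTest is a functional test that checks whether the player character can double jump.
; On test start it sets the character's JumpCount to 2, then calls the character's JumpTest twice every tick.
; The test succeeds when that character begins overlapping the TriggerBox actor; the graph has no explicit failure branch.
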(event OnActorBeginOverlap(TriggerBox)
  (params (OverlappedActor :type Actor%20Object%20Reference) (OtherActor :type Actor%20Object%20Reference))
  (if (== OtherActor (Variables|Default|GetCharacter))
    (Class|FunctionalTest|FinishTest "Succeeded" "Player Succesfully Jumped")))

(event EventPrepareTest)

(event EventStartTest
  (Variables|/Game/Blueprints/Chracter_Blueprint/Paper2DCharacter.Paper2DCharacter_C|SetjumpCount (Variables|Default|GetCharacter) 2))

(event EventTick
  (params (DeltaSeconds :type Float%20%28single-precision%29))
  (bind _character (Variables|Default|GetCharacter))
  (Default|JumpTest _character)
  (Default|JumpTest _character))

(fn ConstructionScript)