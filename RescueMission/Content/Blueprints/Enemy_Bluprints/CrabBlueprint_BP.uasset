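; Crab enemy Blueprint for a flipbook-sprite character that patrols between two points and reacts to a nearby player.
; BeginPlay detaches the patrol point components to fix them in world space, then sets health and damage stats.
; Each Tick runs a distance check: a close player makes it turn and chase while within the patrol X bounds.
; Otherwise it walks to the current target, turning and alternating points via a FlipFlop on arrival.
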(event Custom|CrabDetector
  ;[1 1 1] Player Detection
  (if (< (Math|Vector|Distance(Vector) (Transformation|GetActorLocation (Game|GetPlayerCharacter 0)) (Transformation|GetActorLocation self)) 2e+02)
    (Variables|Default|SetisPlayerNearBy true)
    (else
      (Variables|Default|SetisPlayerNearBy false))))

(event Custom|SetPatrolPoint
  ;[1 1 1] Setting points to patrol between
  (Utilities|FlowControl|FlipFlop
    (:A
      (Variables|Default|SetTargetLoc (Transformation|GetWorldLocation (Variables|Default|GetLeftPatrolPoint))))
    (:B
      (Variables|Default|SetTargetLoc (Transformation|GetWorldLocation (Variables|Default|GetRightPatrolPoint))))))

(event EventTick
  (params (DeltaSeconds :type Float%20%28single-precision%29))
  (bind _returnvalue (Transformation|GetActorLocation))
  (bind _self self)
  (bind _targetloc (Variables|Default|GetTargetLoc))
  (bind _returnvalue_2 (Transformation|GetActorLocation _self))
  (bind _x (Class|KismetMathLibrary|BreakVector3f _returnvalue_2))
  ;[1 1 1] Patrol in between
  (CallFunction|CrabDetector)
  (Sprite|SetFlipbook (Variables|Default|GetSprite) "/Game/Assets/Enemy_Assets/Crab_Enemy/crab-walk/crab-walk.crab-walk")
  (if (Variables|Default|GetisPlayerNearBy)
    (CallFunction|RotateTowardsPlayer)
    ;;[1 1 1] Buraya handle animation gerekçek
    (if (and (< _x (.X (Class|KismetMathLibrary|BreakVector3f (Transformation|GetWorldLocation (Variables|Default|GetRightPatrolPoint))))) (> _x (.X (Class|KismetMathLibrary|BreakVector3f (Transformation|GetWorldLocation (Variables|Default|GetLeftPatrolPoint))))))
      (Pawn|Input|AddMovementInput (Math|Vector|GetUnitDirection(Vector) _returnvalue_2 (Transformation|GetActorLocation (Game|GetPlayerCharacter 0))) 1.0 false))
    (else
      (Pawn|Input|AddMovementInput (Math|Vector|GetUnitDirection(Vector) _returnvalue _targetloc) 1.0 false)
      (if (< (Math|Vector|Distance(Vector) _returnvalue _targetloc) 2.0)
        (if (!= (Variables|Default|GetwasMovingRight) (Variables|Default|GetisMovingRight))
          _
          (else
            (Variables|Default|SetisMovingRight (Variables|Default|GetwasMovingRight))))
        (CallFunction|RotateNew)
        (CallFunction|SetPatrolPoint)))))

(event EventBeginPlay
  (Transformation|DetachFromComponent (Variables|Default|GetLeftPatrolPoint) "KeepWorld" "KeepWorld" "KeepWorld" true)
  (CallFunction|SetPatrolPoint)
  (Variables|Default|SetBase%20Damage 5.0)
  (Variables|Default|SetDamage%20Duration 1.5)
  (Variables|Default|SetHealth 5e+01)
  (|CallParentFunction))

(fn ConstructionScript
  (|CallParentFunction))