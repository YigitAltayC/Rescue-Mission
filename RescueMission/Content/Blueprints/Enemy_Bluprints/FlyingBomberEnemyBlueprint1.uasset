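; Flying bomber enemy that homes in on the player's Paper2D character when close and self-destructs.
; Each Tick checks distance, then either sets the FlyingMovement homing target and counts down to explosion, or stops movement.
; Capsule overlap with the player or BP_Mutated_Character also explodes it, spawning an impact actor, and applies damage to Metroid.
; Box overlap with a SceneCapture2D starts a looping timer that flashes the sprite red.
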(event OnComponentBeginOverlap(Box)
  (params (OverlappedComponent :type Primitive%20Component%20Object%20Reference) (OtherActor :type Actor%20Object%20Reference) (OtherComp :type Primitive%20Component%20Object%20Reference) (OtherBodyIndex :type Integer) (bFromSweep :type Boolean) (SweepResult :type Hit%20Result%20Structure%20%28by%20ref%29))
  (Utilities|Casting|CastToSceneCapture2D OtherActor)
  (Variables|Default|SetSprite%20Color (Class|PaperFlipbookComponent|GetSpriteColor (Variables|Default|GetSprite)))
  (CallFunction|Dot)
  (CallFunction|StartDot))

(event OnComponentBeginOverlap(CapsuleComponent)
  (params (OverlappedComponent :type Primitive%20Component%20Object%20Reference) (OtherActor :type Actor%20Object%20Reference) (OtherComp :type Primitive%20Component%20Object%20Reference) (OtherBodyIndex :type Integer) (bFromSweep :type Boolean) (SweepResult :type Hit%20Result%20Structure%20%28by%20ref%29))
  ;[1 1 1] Explosion on Collision
  (Utilities|Casting|CastToPaper2DCharacter OtherActor
    (:then
      _)
    (:CastFailed
      (Utilities|Casting|CastToBP_Mutated_Character OtherActor)))
  (CallFunction|Explosion)
  (Game|Damage|ApplyDamage (Variables|Default|GetMetroid) (Variables|Default|GetBase%20Damage) 0 0))

(event Custom|Calculate%20Distance%20to%20Player
  ;[1 1 1] Calculate Distance to Player Function
  (bind _aspaper_2dcharacter (Utilities|Casting|CastToPaper2DCharacter (Game|GetPlayerCharacter 0)))
  (if (< (Transformation|GetDistanceTo self _aspaper_2dcharacter) 1e+02)
    (Variables|Default|SetIsDetectingPlayer true)
    (else
      (Variables|Default|SetIsDetectingPlayer false))))

(event Custom|Start%20Dot
  ;[1 1 1] Changing Texture
  (bind _returnvalue (Utilities|Time|SetTimerbyEvent (delegate Custom|Dot) (Variables|Default|GetDuration) true))
  (Variables|Default|SetDot%20Timer _returnvalue))

(event Custom|Dot
  (bind _sprite (Variables|Default|GetSprite))
  ;[1 1 1] Changing Texture
  (Sprite|SetSpriteColor _sprite (Math|Color|MakeColor 1.0 0.0 0.0))
  (Utilities|FlowControl|Delay 0.1)
  (Sprite|SetSpriteColor _sprite (Variables|Default|GetSprite%20Color)))

(event Custom|End%20Dot
  ;[1 1 1] Changing Texture
  (Utilities|Time|ClearandInvalidateTimerbyHandle (Variables|Default|GetDot%20Timer)))

(event EventBeginPlay
  (Variables|Default|SetBase%20Damage 2e+01)
  (Variables|Default|SetExplosion%20Time 2.0)
  (Variables|Default|SetDamage%20Duration 0.5)
  (Variables|Default|SetHealth 4e+01)
  (|CallParentFunction))

(event EventTick
  (params (DeltaSeconds :type Float%20%28single-precision%29))
  ;[1 1 1] Follow Player When On Spesific Bounds + Explosion After 2 Seconds of Movement
  (CallFunction|CalculateDistancetoPlayer)
  (if (Variables|Default|GetIsDetectingPlayer)
    (CallFunction|CountDownExplosionTimer DeltaSeconds)
    (bind _aspaper_2dcharacter (Utilities|Casting|CastToPaper2DCharacter (Game|GetPlayerCharacter 0)))
    (Variables|/Script/Engine.ProjectileMovementComponent|SetHomingTargetComponent (Variables|Default|GetFlyingMovement) (Variables|/Script/Engine.Character|GetCapsuleComponent _aspaper_2dcharacter))
    (if (<= (Variables|Default|GetExplosion%20Time) 0.0)
      (CallFunction|Explosion))
    (else
      (Components|Movement|StopMovementImmediately (Variables|Default|GetFlyingMovement)))))

(fn ConstructionScript
  (|CallParentFunction))

(fn CountDownExplosionTimer
  (params (Delta%20Time :type Float%20%28double-precision%29))
  (Variables|Default|SetExplosion%20Time (- (Variables|Default|GetExplosion%20Time) Delta%20Time)))

(fn Explosion
  (Game|SpawnActorfromClass "/Game/Blueprints/Bullet_and_Impact_Blueprint/Impacts/EnemyMissileImpact_BP.EnemyMissileImpact_BP_C" (Transformation|GetActorTransform self) "Undefined" 0 0)
  (Actor|DestroyActor))