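; Base 2D side-scrolling enemy that walks along X in its current facing direction, pinned to a fixed Y plane each tick.
; Capsule overlap with the player or mutated player starts damage over time using the enemy's base damage and duration, and leaving ends it.
; Incoming damage reddens the sprite and lowers health until a lethal hit spawns EnemyDeath_BP and destroys the actor.
; Helpers provide turning, player-facing and damage scaling.
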(event OnComponentBeginOverlap(CapsuleComponent)
  (params (OverlappedComponent :type Primitive%20Component%20Object%20Reference) (OtherActor :type Actor%20Object%20Reference) (OtherComp :type Primitive%20Component%20Object%20Reference) (OtherBodyIndex :type Integer) (bFromSweep :type Boolean) (SweepResult :type Hit%20Result%20Structure%20%28by%20ref%29))
  (bind _metroid (Variables|Default|GetMetroid))
  ;[1 1 1] Comment
  (bind _playerref (Class|PlayerInterface|PlayerRef(Message) OtherActor))
  (Utilities|IsValid _playerref
    (:Is%20Valid
      _)
    (:Is%20Not%20Valid
      (bind _playerref_2 (Class|MutatedInterface|MutatedPlayerRef(Message) OtherActor))
      (Utilities|IsValid _playerref_2
        (:Is%20Valid
          _))))
  (Variables|/Game/Blueprints/Chracter_Blueprint/Paper2DCharacter.Paper2DCharacter_C|SetDamage%20Recieved _metroid (Variables|Default|GetBase%20Damage))
  (Variables|/Game/Blueprints/Chracter_Blueprint/Paper2DCharacter.Paper2DCharacter_C|SetDuration _metroid (Variables|Default|GetDamage%20Duration))
  (Default|Dot _playerref)
  (Default|StartDot _playerref))

(event OnComponentEndOverlap(CapsuleComponent)
  (params (OverlappedComponent :type Primitive%20Component%20Object%20Reference) (OtherActor :type Actor%20Object%20Reference) (OtherComp :type Primitive%20Component%20Object%20Reference) (OtherBodyIndex :type Integer))
  ;[1 1 1] Comment
  (bind _playerref (Class|PlayerInterface|PlayerRef(Message) OtherActor))
  (Utilities|IsValid _playerref
    (:Is%20Valid
      _)
    (:Is%20Not%20Valid
      (bind _playerref_2 (Class|MutatedInterface|MutatedPlayerRef(Message) OtherActor))
      (Utilities|IsValid _playerref_2
        (:Is%20Valid
          _))))
  (Default|EndDot _playerref))

(event Custom|RotateOld
  (bind _sprite (Variables|Default|GetSprite))
  (bind _returnvalue (Transformation|GetWorldScale _sprite))
  ;[1 1 1] Rotate
  (Transformation|SetWorldScale3D (Variables|Default|GetSprite) (Math|Vector|MakeVector (* (select (Variables|Default|GetisMovingRight) -1.0 1.0) (.x _returnvalue)) (.y _returnvalue) (.z _returnvalue)))
  (if (Variables|Default|GetisMovingRight)
    (Variables|Default|SetisMovingRight false)
    (else
      (Variables|Default|SetisMovingRight true))))

(event Custom|Rotate%20New
  (bind _sprite (Variables|Default|GetSprite))
  (bind _returnvalue (Transformation|GetWorldRotation _sprite))
  (Variables|Default|SetisMovingRight (not (Variables|Default|GetisMovingRight)))
  (Transformation|SetWorldRotation _sprite (Math|Rotator|MakeRotator (.roll _returnvalue) (.pitch _returnvalue) (Math|Float|%(Float) (+ (.yaw _returnvalue) 1.8e+02) 3.6e+02)) false false))

(event Custom|Rotate%20Towards%20Player
  (bind _returnvalue (CallFunction|XDistancetoPlayer))
  (if (> _returnvalue 0.0)
    (if (Variables|Default|GetisMovingRight)
      (Variables|Default|SetwasMovingRight true)
      (CallFunction|RotateNew)
      (else
        (Variables|Default|SetwasMovingRight false)))
    (elif (Variables|Default|GetisMovingRight)
      (Variables|Default|SetwasMovingRight true)
      (else
        (Variables|Default|SetwasMovingRight false)
        (CallFunction|RotateNew)))))

(event Custom|Stuck%20Y
  (bind _returnvalue (Transformation|GetActorLocation))
  ;[1 1 1] Make Sure the Enemy Has Correct Y Axis
  (if (not (== (.y (Transformation|GetWorldLocation (Variables|Default|GetSprite self))) -1.9e+02))
    (Transformation|SetActorLocation (Math|Vector|MakeVector (.x _returnvalue) -1.9e+02 (.z _returnvalue)) false false)))

(event Game|Damage|EventAnyDamage
  (params (Damage :type Float%20%28single-precision%29) (DamageType :type Damage%20Type%20Object%20Reference) (InstigatedBy :type Controller%20Object%20Reference) (DamageCauser :type Actor%20Object%20Reference))
  (bind _returnvalue (/ Damage 1e+02))
  (bind _sprite (Variables|Default|GetSprite))
  (bind _spritecolor (Variables|/Script/Paper2D.PaperFlipbookComponent|GetSpriteColor _sprite))
  (bind (_r _g _b) (Math|Color|BreakColor _spritecolor))
  ;[1 1 1] Handle Damage
  (if (< Damage (Variables|Default|GetHealth))
    (Sprite|SetSpriteColor _sprite (Math|Color|MakeColor 1.0 (- _g _returnvalue) (- _b _returnvalue)))
    (Variables|Default|SetHealth (- (Variables|Default|GetHealth) Damage))
    (else
      (Game|SpawnActorfromClass "/Game/Blueprints/Enemy_Bluprints/EnemyDeath_BP.EnemyDeath_BP_C" (Transformation|GetActorTransform) "Undefined" 0 0)
      (Actor|DestroyActor))))

(event EventTick
  (params (DeltaSeconds :type Float%20%28single-precision%29))
  ;[1 1 1] Enemy Move
  (CallFunction|StuckY)
  (Pawn|Input|AddMovementInput "1.000000, 0, 0" (select (Variables|Default|GetisMovingRight) 1.0 -1.0) false))

(event EventBeginPlay
  ;[1 1 1] Random Move Direction
  (bind _returnvalue (Actor|GetActorOfClass "/Game/Blueprints/Chracter_Blueprint/Paper2DCharacter.Paper2DCharacter_C"))
  (Variables|Default|SetMetroid _returnvalue))

(fn ConstructionScript)

(fn IncreaseBaseDamage
  (Variables|Default|SetBase%20Damage (+ (* (Variables|Default|GetBase%20Damage) 0.1) (Variables|Default|GetBase%20Damage))))

(fn XDistancetoPlayer
  (return (- (.x (Transformation|GetActorLocation self)) (.x (Transformation|GetActorLocation (Game|GetPlayerCharacter 0))))))

(fn GetSpriteFlipbookLength
  (params (Sprite :type Paper%20Flipbook%20Object%20Reference))
  (return (CallFunction|GetSpriteFlipbookLength Sprite)))