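; Projectile enemy Blueprint for a flipbook-based enemy that fires bullets at the player.
; StartShootingPlayer switches to the attack flipbook and starts a looping timer matched to its length, so each BP_EnemyBullet spawns at BulletSpawnPoint as the animation finishes.
; StopShootingPlayer clears the timer and restores the normal flipbook.
; An unconnected arctangent aiming experiment, noted as broken, never runs, so the enemy does not rotate toward the player.
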(event Custom|StartShootingPlayer
  (bind _sprite (Variables|Default|GetSprite))
  ;[1 0.6234 0.4637] shoot player every sequence duraiton
  (Sprite|SetFlipbook _sprite "/Game/Assets/Enemy_Assets/waechter/weachter_attack.weachter_attack")
  (bind _returnvalue (Utilities|Time|SetTimerbyEvent (delegate Custom|FireBullet) (Class|PaperFlipbookComponent|GetFlipbookLength _sprite) true))
  (Variables|Default|Settimer _returnvalue))

(event Custom|FireBullet
  ;[1 0.6234 0.4637] spawn the bullet
  (Game|SpawnActorfromClass "/Game/Blueprints/Bullet_and_Impact_Blueprint/EnemyBullet/BP_EnemyBullet.BP_EnemyBullet_C" (Transformation|GetWorldTransform (Variables|Default|GetBulletSpawnPoint)) "Undefined" 0 0))

(event Custom|StopShootingPlayer
  ;[1 0.6234 0.4637] clear the timer and change the flipbook to normal
  (Utilities|Time|ClearandInvalidateTimerbyHandle (Variables|Default|Gettimer))
  (Sprite|SetFlipbook (Variables|Default|GetSprite) "/Game/Assets/Enemy_Assets/waechter/waechter_normal.waechter_normal"))

(event EventBeginPlay
  (|CallParentFunction))

(event Collision|EventActorBeginOverlap
  (params (OtherActor :type Actor%20Object%20Reference)))

(event EventTick
  (params (DeltaSeconds :type Float%20%28single-precision%29))
  (|CallParentFunction DeltaSeconds) ; This node is disabled and will not be called.\nDrag off pins to build functionality.
)

(fn ConstructionScript
  (|CallParentFunction))