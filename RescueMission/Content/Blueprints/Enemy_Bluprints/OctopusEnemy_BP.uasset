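; Octopus enemy for a Paper2D game that patrols and attacks the player, building on a parent enemy Blueprint.
; Tick walks it between two detached points, flipping at each end and pausing while the player is in range.
; Box overlap turns it toward the player and spawns a missile impact with debug prints; capsule overlap fires a bullet.
; Timer-driven shooting events synced to flipbook length exist but are not called within this graph.
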(event OnComponentBeginOverlap(CapsuleComponent)
  (params (OverlappedComponent :type Primitive%20Component%20Object%20Reference) (OtherActor :type Actor%20Object%20Reference) (OtherComp :type Primitive%20Component%20Object%20Reference) (OtherBodyIndex :type Integer) (bFromSweep :type Boolean) (SweepResult :type Hit%20Result%20Structure%20%28by%20ref%29))
  (Utilities|Casting|CastToPaper2DCharacter OtherActor)
  (Game|SpawnActorfromClass "/Game/Blueprints/Bullet_and_Impact_Blueprint/EnemyBullet/BP_EnemyBullet.BP_EnemyBullet_C" (Transformation|GetWorldTransform (Variables|Default|GetBulletSpawnPoint)) "Undefined" 0 0))

(event OnComponentBeginOverlap(Box1)
  (params (OverlappedComponent :type Primitive%20Component%20Object%20Reference) (OtherActor :type Actor%20Object%20Reference) (OtherComp :type Primitive%20Component%20Object%20Reference) (OtherBodyIndex :type Integer) (bFromSweep :type Boolean) (SweepResult :type Hit%20Result%20Structure%20%28by%20ref%29))
  (bind _bulletspawnpoint (Variables|Default|GetBulletSpawnPoint))
  (Utilities|Casting|CastToPaper2DCharacter OtherActor)
  (bind _is_player_on_right (CallFunction|IsPlayeronRight (Transformation|GetActorLocation (Game|GetPlayerCharacter 0)) (Transformation|GetActorLocation self)))
  (if (!= _is_player_on_right (Variables|Default|GetisMovingRight))
    (CallFunction|RotateTowardsPlayer)
    (Transformation|SetWorldLocation _bulletspawnpoint (* (Transformation|GetWorldLocation _bulletspawnpoint) "-1.000000,0.000000,0") false false))
  (Game|SpawnActorfromClass "/Game/Blueprints/Bullet_and_Impact_Blueprint/Impacts/MissileImpact_BP.MissileImpact_BP_C" (Transformation|GetWorldTransform _bulletspawnpoint) "Undefined" 0 0)
  (Development|PrintString (Utilities|String|ToString(Transform) (Transformation|GetActorTransform self)))
  (Development|PrintString "Hello"))

(event Custom|StartShootingPlayer
  (bind _sprite (Variables|Default|GetSprite))
  (Sprite|SetFlipbook _sprite "/Game/Assets/Enemy_Assets/Octopus_Enemy/octopus/octopus.octopus")
  (bind _returnvalue (Utilities|Time|SetTimerbyEvent (delegate Custom|FireBullet) (Class|PaperFlipbookComponent|GetFlipbookLength _sprite) true))
  (Variables|Default|Settimer _returnvalue))

(event Custom|SetPatrolPoint
  ;[1 1 1] Setting points to patrol between
  (Utilities|FlowControl|FlipFlop
    (:A
      (Variables|Default|SetTargetLoc (Transformation|GetWorldLocation (Variables|Default|GetLeftPatrolPoint))))
    (:B
      (Variables|Default|SetTargetLoc (Transformation|GetWorldLocation (Variables|Default|GetRightPatrolPoint))))))

(event Custom|FireBullet
  ;[1 0.6234 0.4637] spawn the bullet
  (Game|SpawnActorfromClass "/Game/Blueprints/Bullet_and_Impact_Blueprint/EnemyBullet/BP_EnemyBullet.BP_EnemyBullet_C" (Transformation|GetWorldTransform (Variables|Default|GetBulletSpawnPoint)) "Undefined" 0 0))

(event Custom|StopShootingPlayer
  ;[1 0.6234 0.4637] clear the timer and change the flipbook to normal
  (Utilities|Time|ClearandInvalidateTimerbyHandle (Variables|Default|Gettimer))
  (Sprite|SetFlipbook (Variables|Default|GetSprite) "/Game/Assets/Enemy_Assets/Octopus_Enemy/octopus/octopus.octopus"))

(event Custom|Patrol%20In%20Between
  (bind _returnvalue (Transformation|GetActorLocation))
  (bind _targetloc (Variables|Default|GetTargetLoc))
  (bind _bulletspawnpoint (Variables|Default|GetBulletSpawnPoint))
  (bind _player_in_range (CallFunction|PlayerDetector 2e+02 (Transformation|GetActorLocation (Game|GetPlayerCharacter 0)) (Transformation|GetActorLocation self)))
  (if (not _player_in_range)
    (Pawn|Input|AddMovementInput (Math|Vector|GetUnitDirection(Vector) _returnvalue _targetloc) 1.0 false)
    (if (< (Math|Vector|Distance(Vector) _returnvalue _targetloc) 2.0)
      (if (!= (Variables|Default|GetwasMovingRight) (Variables|Default|GetisMovingRight))
        _
        (else
          (Variables|Default|SetisMovingRight (Variables|Default|GetwasMovingRight))))
      (CallFunction|RotateNew)
      (Transformation|SetWorldLocation _bulletspawnpoint (* (Transformation|GetWorldLocation _bulletspawnpoint) "-1.000000,0.000000,0") false false)
      (CallFunction|SetPatrolPoint))))

(event EventTick
  (params (DeltaSeconds :type Float%20%28single-precision%29))
  (CallFunction|PatrolinBetween))

(event EventBeginPlay
  (Transformation|DetachFromComponent (Variables|Default|GetLeftPatrolPoint) "KeepWorld" "KeepWorld" "KeepWorld" true)
  (CallFunction|SetPatrolPoint)
  (Variables|Default|SetBase%20Damage 1e+01)
  (Variables|Default|SetDamage%20Duration 1.5)
  (Variables|Default|SetHealth 2e+02)
  (|CallParentFunction))

(fn ConstructionScript
  (|CallParentFunction))

(fn PlayerDetector
  (params (Range :type Float%20%28double-precision%29) (Player%20Location :type Vector) (Enemy%20Location :type Vector))
  (if (< (Math|Vector|Distance(Vector) Player%20Location Enemy%20Location) Range)
    (return true)
    (else
      (return false))))

(fn IsPlayeronRight
  (params (Player%20Location :type Vector) (Enemy%20Location :type Vector))
  (if (< (- (.x Player%20Location) (.x Enemy%20Location)) 0.0)
    (return false)
    (else
      (return true))))