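; Flying enemy Blueprint that chases the player's Paper2D character at close range and damages it on contact.
; Each tick, a distance check sets a detection flag, which either sets the player's capsule as the homing target of FlyingMovement or stops movement immediately.
; The enemy's capsule overlap applies damage to any Paper2D character it touches.
; BeginPlay initializes health and damage variables, which are not read in these graphs.
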(event OnComponentBeginOverlap(CapsuleComponent)
  (params (OverlappedComponent :type Primitive%20Component%20Object%20Reference) (OtherActor :type Actor%20Object%20Reference) (OtherComp :type Primitive%20Component%20Object%20Reference) (OtherBodyIndex :type Integer) (bFromSweep :type Boolean) (SweepResult :type Hit%20Result%20Structure%20%28by%20ref%29))
  (bind _aspaper_2dcharacter (Utilities|Casting|CastToPaper2DCharacter OtherActor))
  (Game|Damage|ApplyDamage _aspaper_2dcharacter 1.0 0 0))

(event Custom|Calculate%20Distance%20to%20Player
  ;[1 1 1] Calculate Distance to Player Function
  (bind _aspaper_2dcharacter (Utilities|Casting|CastToPaper2DCharacter (Game|GetPlayerCharacter 0)))
  (if (< (Transformation|GetDistanceTo self _aspaper_2dcharacter) 1e+02)
    (Variables|Default|SetIsDetectingPlayer true)
    (else
      (Variables|Default|SetIsDetectingPlayer false))))

(event EventBeginPlay
  (Variables|Default|SetBase%20Damage 1.0)
  (Variables|Default|SetDamage%20Duration 0.5)
  (Variables|Default|SetHealth 4e+01)
  (|CallParentFunction))

(event EventTick
  (params (DeltaSeconds :type Float%20%28single-precision%29))
  ;[1 1 1] Follow Player When On Spesific Bounds
  (CallFunction|CalculateDistancetoPlayer)
  (if (Variables|Default|GetIsDetectingPlayer)
    (bind _aspaper_2dcharacter (Utilities|Casting|CastToPaper2DCharacter (Game|GetPlayerCharacter 0)))
    (Variables|/Script/Engine.ProjectileMovementComponent|SetHomingTargetComponent (Variables|Default|GetFlyingMovement) (Variables|/Script/Engine.Character|GetCapsuleComponent _aspaper_2dcharacter))
    (else
      (Components|Movement|StopMovementImmediately (Variables|Default|GetFlyingMovement)))))

(fn ConstructionScript
  (|CallParentFunction))