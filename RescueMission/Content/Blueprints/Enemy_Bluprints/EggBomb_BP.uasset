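; EggBomb_BP is an egg trap that deals instant and lingering damage when the player steps on it.
; A one-shot box overlap counts the step on the player, applies initial damage, then starts the player's timed damage effect.
; If the player's trap count exceeds one, that effect is delayed until the current one should end.
; Egg and acid-ring flipbooks play alongside, leaving a popped-egg sprite and removing the ring.
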(event OnComponentBeginOverlap(Box)
  (params (OverlappedComponent :type Primitive%20Component%20Object%20Reference) (OtherActor :type Actor%20Object%20Reference) (OtherComp :type Primitive%20Component%20Object%20Reference) (OtherBodyIndex :type Integer) (bFromSweep :type Boolean) (SweepResult :type Hit%20Result%20Structure%20%28by%20ref%29))
  (bind _paperflipbook (Variables|Default|GetPaperFlipbook))
  (bind _acissplatring (Variables|Default|GetAcisSplatRing))
  (bind _playerref (Class|PlayerInterface|PlayerRef(Message) OtherActor))
  (Utilities|IsValid _playerref
    (:Is%20Valid
      (Variables|Default|SethasPlayerSteped true)
      (bind _result (Math|Integer|IncrementInt (Variables|/Game/Blueprints/Chracter_Blueprint/Paper2DCharacter.Paper2DCharacter_C|GetsteppedTrapCount _playerref))
        (:%20%20
          (Variables|/Game/Blueprints/Chracter_Blueprint/Paper2DCharacter.Paper2DCharacter_C|SetsteppedTrapCount _playerref _result)
          (Components|DestroyComponent (Variables|Default|GetBox))
          (Utilities|FlowControl|Sequence
            (:then_0
              ;[1 0.6234 0.4637] apply player initial damage and constant damage for some time
              (Game|Damage|ApplyDamage _playerref (Variables|PlayerDamage|GetInitialDamageAmount) 0 0)
              ;[0.1672 0.2024 1] if player has stepped on the trap while the damage from other trap exists it will delay to ensure that the new traps continuous damage will be applied.
              (if (> (Variables|/Game/Blueprints/Chracter_Blueprint/Paper2DCharacter.Paper2DCharacter_C|GetsteppedTrapCount _playerref) 1)
                (Utilities|FlowControl|Delay (- (Variables|PlayerDamage|GetTotalDamageDuraiton) (Variables|/Game/Blueprints/Chracter_Blueprint/Paper2DCharacter.Paper2DCharacter_C|GetcurrentTime _playerref))))
              (Default|ApplyConstantDamagetoPlayer _playerref (Variables|PlayerDamage|GetFuncitonCallRepeatDuration) (Variables|PlayerDamage|GetDamageAmount) (Variables|PlayerDamage|GetTotalDamageDuraiton)))
            (:then_1
              ;[1 0.6234 0.4637] play explosion animation on egg
              (Sprite|SetFlipbook _paperflipbook "/Game/Assets/Enemy_Assets/Egg_Bomb_Enemy/Egg_Bomb_Explosion.Egg_Bomb_Explosion")
              (Audio|Components|Audio|Play _paperflipbook)
              ;[1 0.6234 0.4637] play explosion animation on ring
              (Sprite|SetFlipbook _acissplatring "/Game/Assets/Enemy_Assets/Egg_Bomb_Enemy/Toxic_Explosion_Effect.Toxic_Explosion_Effect")
              (Audio|Components|Audio|Play _acissplatring))))))))

(event OnFinishedPlaying(PaperFlipbook)
  ;[1 0.6234 0.4637] Change the sprite when animation finishes
  (if (Variables|Default|GethasPlayerSteped)
    (Rendering|Components|Sprite|SetSprite (Variables|Default|GetEggCluster_Sprite) "/Game/Assets/Enemy_Assets/Egg_Bomb_Enemy/EggPopped_Sprite.EggPopped_Sprite")))

(event OnFinishedPlaying(AcisSplatRing)
  ;[1 0.6234 0.4637] Destroy the acid ring
  (if (Variables|Default|GethasPlayerSteped)
    (Components|DestroyComponent (Variables|Default|GetAcisSplatRing))))

(event EventBeginPlay
  (Components|Timeline|SetLooping (Variables|Default|GetPaperFlipbook) false)
  (Components|Timeline|SetLooping (Variables|Default|GetAcisSplatRing) false))

(event Collision|EventActorBeginOverlap
  (params (OtherActor :type Actor%20Object%20Reference)))

(fn ConstructionScript)