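; Base Blueprint for 2D Paper bosses, leaving Movement and AttackAction empty for child classes to implement.
; Each Tick checks player distance: detection enters the moving state and advances BP_GameMusic's boss soundtrack, while losing the player deactivates the boss.
; A state machine calls Movement every frame while moving and AttackAction once per entry into attacking.
; Helper functions provide random attack selection, flipbook lookup, axis distances, flipping toward the player and health reduction.
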(event Custom|Calculate%20Distance%20to%20Player
  ;[0.07628 0.25 0.1056] Calculate Distance to Player Event
  (bind _aspaper_2dcharacter (Utilities|Casting|CastToPaper2DCharacter (Game|GetPlayerCharacter 0)))
  (if (< (Transformation|GetDistanceTo self _aspaper_2dcharacter) (Variables|Default|GetPlayer%20Detection%20Range))
    (Variables|Default|SetIs%20Detecting%20Player true)
    (else
      (Variables|Default|SetIs%20Detecting%20Player false))))

(event Custom|Movement
  ;[0 0 0] Abstract Methods
  ;
  ; Please do not try to write its functions in here, they will be only implemented in the children classes.
)

(event Custom|Attack%20Action
  ;[0 0 0] Abstract Methods
  ;
  ; Please do not try to write its functions in here, they will be only implemented in the children classes.
)

(event EventTick
  (params (DeltaSeconds :type Float%20%28single-precision%29))
  (CallFunction|CalculateDistancetoPlayer)
  (if (Variables|Default|GetIs%20Detecting%20Player)
    ;[0.1686 0.1882 0.06274] Activate Boss' Movement by Setting Its State to Moving State, If Player gets detected from the boss and state hasn't been set
    (if (not (Variables|Default|GetState%20Set))
      (Variables|Default|SetCurrent%20State "NewEnumerator0")
      (Variables|Default|SetState%20Set true)
      (Default|PlayNextBossSoundtrack (Variables|Default|GetGame%20Music%20Reference))
      (else
        ;[0.1686 0.1882 0.06274] Boss State Machine
        (switch Utilities|FlowControl|Switch|SwitchonBossState (Variables|Default|GetCurrent%20State)
          (:NewEnumerator0
            (Variables|Default|SetHas%20Entered%20Attack%20State false)
            (CallFunction|Movement))
          (:NewEnumerator1
            (if (not (Variables|Default|GetHas%20Entered%20Attack%20State))
              (Variables|Default|SetHas%20Entered%20Attack%20State true)
              (CallFunction|AttackAction))))))
    (else
      ;[0.1686 0.1882 0.06274] Disable Boss by Setting Its State to Non-Active State If player hasn't been detected by the boss
      (Variables|Default|SetCurrent%20State "NewEnumerator3")
      (Variables|Default|SetState%20Set false))))

(event EventBeginPlay
  ;[0.08527 0.04373 0.2708] Setting Up Variables
  (bind _outactors (Actor|GetAllActorsOfClass "/Game/MusicAndSfx/BP_GameMusic.BP_GameMusic_C"))
  (Variables|Default|SetGame%20Music%20Reference (Utilities|Array|Get(acopy) _outactors))
  (Variables|Default|SetAttackTypeCount (Utilities|Array|Length (Variables|Default|GetBoss%20Attacks))))

(fn ConstructionScript)

(fn GetXDistancetoPlayer
  (return (- (.x (Transformation|GetActorLocation self)) (.x (Transformation|GetActorLocation (Game|GetPlayerCharacter 0))))))

(fn GetRandomAttack
  (return (Math|Random|RandomInteger (Variables|Default|GetAttackTypeCount))))

(fn GetAttackSprite
  (params (Index :type Integer))
  (return (.PaperFlipbook (Utilities|Struct|BreakBPS_BossAttack (Utilities|Array|Get(acopy) (Variables|Default|GetBoss%20Attacks) Index)))))

(fn GetXDistancetoPoint
  (params (Point :type Static%20Mesh%20Component%20Object%20Reference))
  (return (- (.x (Transformation|GetWorldLocation Point)) (.x (Transformation|GetActorLocation self)))))

(fn GetAttackSpriteLooping
  (params (Index :type Integer))
  (return (.IsLooping (Utilities|Struct|BreakBPS_BossAttack (Utilities|Array|Get(acopy) (Variables|Default|GetBoss%20Attacks) Index)))))

(fn Flip
  (params (Look%20Left :type Boolean))
  (bind _returnvalue (CallFunction|GetXDistancetoPlayer))
  (CallFunction|CalculateDistancetoPlayer)
  (if (Variables|Default|GetIs%20Detecting%20Player)
    (bind _output_get (LocalVariables|SetLocal%20Look%20Left Look%20Left))
    (if _output_get
      (if (> _returnvalue 0.0)
        (bind _output_get_2 (LocalVariables|SetLocal%20Look%20Left (not (LocalVariables|GetLocal%20Look%20Left)) :!label _label))
        (Class|Actor|AddActorWorldRotation "0,180.000000, 0")
        (return _output_get_2))
      (elif (< _returnvalue 0.0)
        (goto _label)))))

(fn DecreaseHealth
  (params (Damage :type Float%20%28double-precision%29))
  (Variables|Default|SetHealth (- (Variables|Default|GetHealth) Damage)))

(fn GetZDistancetoPlayer
  (return (- (.z (Transformation|GetActorLocation self)) (.z (Transformation|GetActorLocation (Game|GetPlayerCharacter 0))))))