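; Laser beam attack actor for the Golem boss that damages the player over time while they overlap it.
; On spawn it plays a laser sound and destroys itself after a set lifetime.
; Its collision box gets the player through PlayerRefMessage, passes damage and duration to the player's own DoT logic and starts it.
; Leaving the box ends that DoT.
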(event OnComponentBeginOverlap(CollisionBox)
  (params (OverlappedComponent :type Primitive%20Component%20Object%20Reference) (OtherActor :type Actor%20Object%20Reference) (OtherComp :type Primitive%20Component%20Object%20Reference) (OtherBodyIndex :type Integer) (bFromSweep :type Boolean) (SweepResult :type Hit%20Result%20Structure%20%28by%20ref%29))
  (bind _playerref (Class|PlayerInterface|PlayerRef(Message) OtherActor))
  (Utilities|IsValid _playerref
    (:Is%20Valid
      (Variables|Default|SetTarget%20Player _playerref)
      (Variables|/Game/Blueprints/Chracter_Blueprint/Paper2DCharacter.Paper2DCharacter_C|SetDamage%20Recieved (Variables|Default|GetTarget%20Player) (Variables|Default|GetBase%20Damage))
      (Variables|/Game/Blueprints/Chracter_Blueprint/Paper2DCharacter.Paper2DCharacter_C|SetDuration (Variables|Default|GetTarget%20Player) (Variables|Default|GetDamage%20Duration))
      (Default|Dot (Variables|Default|GetTarget%20Player))
      (Default|StartDot (Variables|Default|GetTarget%20Player)))))

(event OnComponentEndOverlap(CollisionBox)
  (params (OverlappedComponent :type Primitive%20Component%20Object%20Reference) (OtherActor :type Actor%20Object%20Reference) (OtherComp :type Primitive%20Component%20Object%20Reference) (OtherBodyIndex :type Integer))
  (bind _playerref (Class|PlayerInterface|PlayerRef(Message) OtherActor))
  (Utilities|IsValid _playerref
    (:Is%20Valid
      (Default|EndDot _playerref))))

(event EventBeginPlay
  (Audio|PlaySound2D "/Game/MusicAndSfx/BossMusicAndSFX/laser_Cue.laser_Cue" 1.0 1.0 0.0 0 0)
  (Utilities|FlowControl|Delay (Variables|Default|GetLifetime%20Duration))
  (Actor|DestroyActor))

(event Collision|EventActorBeginOverlap
  (params (OtherActor :type Actor%20Object%20Reference)))

(event EventTick
  (params (DeltaSeconds :type Float%20%28single-precision%29)))

(fn ConstructionScript)