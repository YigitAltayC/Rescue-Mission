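; Golem boss with flipbook sprites that alternates timed random horizontal movement with randomly chosen attacks, building on parent boss logic.
; Attacks are a teleport punch with an enlarged hit capsule, a chain of ground shocks from a side point, and a laser beam.
; Capsule overlap damages and launches the player.
; Zero health triggers death: repeated explosions, boss music ends, and a corpse actor replaces the boss.
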(event OnComponentBeginOverlap(CapsuleCollision)
  (params (OverlappedComponent :type Primitive%20Component%20Object%20Reference) (OtherActor :type Actor%20Object%20Reference) (OtherComp :type Primitive%20Component%20Object%20Reference) (OtherBodyIndex :type Integer) (bFromSweep :type Boolean) (SweepResult :type Hit%20Result%20Structure%20%28by%20ref%29))
  (if (not (Variables|Default|GetIs%20Overlapping))
    (Variables|Default|SetIs%20Overlapping true)
    (bind _playerref (Class|PlayerInterface|PlayerRef(Message) OtherActor))
    (Utilities|IsValid _playerref
      (:Is%20Valid
        (Variables|Default|SetTarget%20Player _playerref)
        (if (Variables|Default|GetIs%20Punching)
          (Game|Damage|ApplyDamage (Variables|Default|GetTarget%20Player) (.DamageAmount (Utilities|Struct|BreakBPS_BossAttack (Utilities|Array|Get(acopy) (Variables|Default|GetBoss%20Attacks)))) 0 0)
          (else
            (Game|Damage|ApplyDamage (Variables|Default|GetTarget%20Player) 2e+01 0 0)))
        (if (Variables|ForFlipping|GetLook%20Left)
          (Character|LaunchCharacter (Variables|Default|GetTarget%20Player) "1000.000000, 0,0.000000" false false)
          (else
            (Character|LaunchCharacter (Variables|Default|GetTarget%20Player) "-1000.000000, 0,0.000000" false false)))))))

(event OnComponentEndOverlap(CapsuleCollision)
  (params (OverlappedComponent :type Primitive%20Component%20Object%20Reference) (OtherActor :type Actor%20Object%20Reference) (OtherComp :type Primitive%20Component%20Object%20Reference) (OtherBodyIndex :type Integer))
  (Variables|Default|SetIs%20Overlapping false))

(event Custom|Death%20Explosion%20Spawn
  (bind _returnvalue (Transformation|GetActorTransform))
  (Game|SpawnActorfromClass "/Game/Blueprints/Bullet_and_Impact_Blueprint/Impacts/BP_GolemBossImpact.BP_GolemBossImpact_C" (Math|Transform|MakeTransform (Math|Vector|MakeVector (Math|Random|RandomFloatinRange (+ (.x (.location _returnvalue)) -25.0) (+ (.x (.location _returnvalue)) 25.0)) (+ (.y (.location _returnvalue)) 1e+01) (Math|Random|RandomFloatinRange (+ (.z (.location _returnvalue)) -25.0) (+ (.z (.location _returnvalue)) 25.0))) "0, 0, 0" "1.000000,1.000000,1.000000") "Undefined" 0 0 :!label _label)
  (Utilities|FlowControl|Delay 0.25)
  (bind _result (Math|Integer|IncrementInt (Variables|Default|GetExplosion%20Spawn%20Count))
    (:%20%20
      (if true
        (goto _label)))))

(event Custom|Teleport%20Attack%20and%20Punch
  (bind _returnvalue (Game|GetPlayerCharacter 0))
  (bind _returnvalue_2 (Transformation|GetActorLocation _returnvalue))
  (CallFunction|CalculateDistancetoPlayer)
  (if (Variables|Default|GetIs%20Detecting%20Player)
    (Variables|Attack-PunchAttack|SetTeleport%20Punch%20Location (Math|Vector|MakeVector (+ (Math|Float|SelectFloat 7e+01 -7e+01 (Variables|ForFlipping|GetLook%20Left)) (.x _returnvalue_2)) (.y _returnvalue_2) (.z _returnvalue_2)))
    (CallFunction|AttackPreperationAnimation)
    (Transformation|SetActorLocation (Variables|Attack-PunchAttack|GetTeleport%20Punch%20Location) false false)
    (Utilities|FlowControl|Delay 0.5)
    (Variables|Default|SetIs%20Punching true)
    (Sprite|SetFlipbook (Variables|Default|GetSprite) (CallFunction|GetAttackSprite))
    (Utilities|FlowControl|Delay 0.2)
    (Transformation|SetRelativeTransform (Variables|Default|GetCapsule%20Collision) (Math|Transform|MakeTransform "0, 0, 0" "0, 0, 0" "2.000000,2.000000,2.000000") false false)
    (Utilities|FlowControl|Delay (- (Class|PaperFlipbookComponent|GetFlipbookLength (Variables|Default|GetSprite)) 0.2))
    (Sprite|SetFlipbook (Variables|Default|GetSprite) "/Game/Assets/Enemy_Assets/Mecha-stone_Golem_0_1/PNG_sheet/GolemIdle.GolemIdle")
    (Transformation|SetRelativeTransform (Variables|Default|GetCapsule%20Collision) (Math|Transform|MakeTransform "0, 0, 0" "0, 0, 0" "1.200000,1.200000,1.200000") false false)
    (Variables|Default|SetCurrent%20State "NewEnumerator0")
    (Variables|Default|SetIs%20Punching false)))

(event Custom|Attack%20Preperation%20Animation
  (Audio|PlaySoundatLocation "/Game/MusicAndSfx/BossMusicAndSFX/teleport_Cue.teleport_Cue" (Transformation|GetActorLocation) "0, 0, 0" 1.0 1.0 0.0 0 0 0 0)
  (Components|Movement|StopMovementImmediately (Variables|Character|GetCharacterMovement))
  (Sprite|SetFlipbook (Variables|Default|GetSprite) "/Game/Assets/Enemy_Assets/Mecha-stone_Golem_0_1/PNG_sheet/GolemPreparingTPAttack.GolemPreparingTPAttack")
  (Utilities|FlowControl|Delay (Class|PaperFlipbookComponent|GetFlipbookLength (Variables|Default|GetSprite))))

(event Custom|Spawn%20Ground%20Shocks
  (bind _returnvalue (Transformation|GetActorLocation))
  (Variables|Attack-ShockAttack|SetShock%20Attack%20Spawned%20Count 1)
  (bind _x (CallFunction|GenerateShockAttackXPosition :!label _label))
  (bind _returnvalue_2 (Game|SpawnActorfromClass "/Game/Blueprints/Enemy_Bluprints/Bosses/GolemBoss/GroundShockAttack.GroundShockAttack_C" (Math|Transform|MakeTransform (Math|Vector|MakeVector _x (- (.y _returnvalue) 4e+01) (- (.z _returnvalue) 6e+01)) "0, 0, 0" "1.000000,1.000000,1.000000") "Undefined" 0 0))
  (Default|SetBossBaseAttack _returnvalue_2 (.DamageAmount (Utilities|Struct|BreakBPS_BossAttack (Utilities|Array|Get(acopy) (Variables|Default|GetBoss%20Attacks) 1))))
  (Variables|Attack-ShockAttack|SetSpawned%20Ground%20Shock%20Attack _returnvalue_2)
  (if (<= (Variables|Attack-ShockAttack|GetShock%20Attack%20Spawned%20Count) (Variables|Attack-ShockAttack|GetShock%20Attack%20Max%20Spawn%20Count))
    (Math|Integer|IncrementInt (Variables|Attack-ShockAttack|GetShock%20Attack%20Spawned%20Count)
      (:%20%20
        (Utilities|FlowControl|Delay (Default|GetLifetimeLength (Variables|Attack-ShockAttack|GetSpawned%20Ground%20Shock%20Attack)))
        (goto _label)))))

(event Custom|Fire%20Laser%20Beam
  (bind _laser_beam___fire_point (Variables|Default|GetLaser%20Beam%20-%20Fire%20Point))
  (bind _returnvalue (Transformation|GetWorldLocation _laser_beam___fire_point))
  (CallFunction|AttackPreperationAnimation)
  (if (Variables|ForFlipping|GetLook%20Left)
    (Game|SpawnActorfromClass "/Game/Blueprints/Enemy_Bluprints/Bosses/GolemBoss/BP_LaserBeamAttack.BP_LaserBeamAttack_C" (Math|Transform|MakeTransform _returnvalue "0, 0, 0" "1.000000,1.000000,1.000000") "Undefined" 0 0)
    (else
      (Game|SpawnActorfromClass "/Game/Blueprints/Enemy_Bluprints/Bosses/GolemBoss/BP_LaserBeamAttack.BP_LaserBeamAttack_C" (Math|Transform|MakeTransform _returnvalue "0,-180.000000, 0" "1.000000,1.000000,1.000000") "Undefined" 0 0)))
  (Sprite|SetFlipbook (Variables|Default|GetSprite) (CallFunction|GetAttackSprite 2))
  (Utilities|FlowControl|Delay 3.0)
  (Sprite|SetFlipbook (Variables|Default|GetSprite) "/Game/Assets/Enemy_Assets/Mecha-stone_Golem_0_1/PNG_sheet/GolemIdle.GolemIdle")
  (Variables|Default|SetCurrent%20State "NewEnumerator0"))

(event Custom|Ground%20Shock%20Attack
  (switch int (Math|Conversions|ToInteger(Boolean) (Math|Random|RandomBool))
    (:0
      (Transformation|SetActorLocation (Transformation|GetWorldLocation (Variables|Default|GetLeft%20-%20Special%20Attack%20Point)) false false))
    (:1
      (Transformation|SetActorLocation (Transformation|GetWorldLocation (Variables|Default|GetRight%20-%20Special%20Attack%20Point)) false false)))
  (Utilities|FlowControl|Delay 0.5)
  (Components|Movement|StopMovementImmediately (Variables|Character|GetCharacterMovement))
  (Utilities|FlowControl|Delay 0.5)
  (Sprite|SetFlipbook (Variables|Default|GetSprite) (CallFunction|GetAttackSprite 1))
  (Utilities|FlowControl|Delay (Class|PaperFlipbookComponent|GetFlipbookLength (Variables|Default|GetSprite)))
  (Sprite|SetFlipbook (Variables|Default|GetSprite) "/Game/Assets/Enemy_Assets/Mecha-stone_Golem_0_1/PNG_sheet/Character_sheet_GolemGroundAttack.Character_sheet_GolemGroundAttack")
  (CallFunction|SpawnGroundShocks)
  (Utilities|FlowControl|Delay 3.0)
  (Sprite|SetFlipbook (Variables|Default|GetSprite) "/Game/Assets/Enemy_Assets/Mecha-stone_Golem_0_1/PNG_sheet/GolemIdle.GolemIdle")
  (Variables|Default|SetCurrent%20State "NewEnumerator0"))

(event Custom|Death
  (bind _returnvalue (Transformation|GetActorTransform))
  (CallFunction|DeathExplosionSpawn)
  (Variables|Default|SetCurrent%20State "NewEnumerator3")
  (Sprite|SetFlipbook (Variables|Default|GetSprite) "/Game/Assets/Enemy_Assets/Mecha-stone_Golem_0_1/PNG_sheet/GolemDeath.GolemDeath")
  (Default|EndBossMusic (Variables|Default|GetGame%20Music%20Reference))
  (Utilities|FlowControl|Delay (Class|PaperFlipbookComponent|GetFlipbookLength (Variables|Default|GetSprite)))
  (Actor|DestroyActor)
  (Game|SpawnActorfromClass "/Game/Blueprints/Enemy_Bluprints/Bosses/GolemBoss/BP_GolemDeadBody.BP_GolemDeadBody_C" (Math|Transform|MakeTransform (Math|Vector|MakeVector (.x (.location _returnvalue)) (- (.y (.location _returnvalue)) 4e+01) (- (.z (.location _returnvalue)) 2e+01)) (.rotation _returnvalue) "2.000000,2.000000,2.000000") "Undefined" 0 0))

(event Collision|EventActorBeginOverlap
  (params (OtherActor :type Actor%20Object%20Reference))
  (|CallParentFunction OtherActor) ; This node is disabled and will not be called.\nDrag off pins to build functionality.
)

(event EventTick
  (params (DeltaSeconds :type Float%20%28single-precision%29))
  (Variables|Default|SetDelta%20Seconds DeltaSeconds)
  (if (> (Variables|Default|GetHealth) 0.0)
    (bind _new_look_left (CallFunction|Flip (Variables|ForFlipping|GetLook%20Left)))
    (Variables|ForFlipping|SetLook%20Left _new_look_left)
    (|CallParentFunction (Variables|Default|GetDelta%20Seconds))
    (elif (not (Variables|Default|GetIs%20Dying))
      (Variables|Default|SetIs%20Dying true)
      (Default|CallBossDied)
      (CallFunction|Death))))

(event EventMovement
  (bind _newparam (CallFunction|GenerateXMovementVector :!label _label))
  (Pawn|Input|AddMovementInput _newparam 5.0 false)
  (Utilities|FlowControl|Delay 0.1)
  (bind _output_get (Variables|Movement|SetTotal%20Movement%20State%20Seconds (+ (Variables|Movement|GetTotal%20Movement%20State%20Seconds) 0.1)))
  (if (<= _output_get (Variables|Movement|GetMovement%20Seconds%20Limit))
    (if (Utilities|Enum|Equal(Enum) (Variables|Default|GetCurrent%20State) "NewEnumerator0")
      (goto _label))
    (else
      (Variables|Default|SetCurrent%20State "NewEnumerator1")
      (Variables|Movement|SetTotal%20Movement%20State%20Seconds 0.0))))

(event Game|Damage|EventAnyDamage
  (params (Damage :type Float%20%28single-precision%29) (DamageType :type Damage%20Type%20Object%20Reference) (InstigatedBy :type Controller%20Object%20Reference) (DamageCauser :type Actor%20Object%20Reference))
  (CallFunction|DecreaseHealth Damage))

(event EventBeginPlay
  ;[0 0 0] Event Begin Play
  (Variables|Default|SetHealth 1e+03)
  (Utilities|FlowControl|Sequence
    (:then_0
      (Variables|Default|SetPlayer%20Detection%20Range 5.5e+02))
    (:then_1
      (CallFunction|CalculateDistancetoPlayer)
      (if (Variables|Default|GetIs%20Detecting%20Player)
        (Variables|Default|SetCurrent%20State "NewEnumerator0")
        (else
          (Variables|Default|SetCurrent%20State "NewEnumerator3"))))
    (:then_2
      (Transformation|DetachFromComponent (Variables|Default|GetLeft%20-%20Special%20Attack%20Point) "KeepWorld" "KeepWorld" "KeepWorld" true)
      (|CallParentFunction))))

(event EventAttackAction
  (switch int (CallFunction|GetRandomAttack)
    (:0
      (CallFunction|TeleportAttackandPunch))
    (:1
      (CallFunction|GroundShockAttack))
    (:2
      (CallFunction|FireLaserBeam))))

(fn ConstructionScript
  (|CallParentFunction))

(fn SetPatrolPoint)

(fn GenerateXMovementVector
  (return (Math|Vector|MakeVector (Math|Random|RandomFloatinRange -1e+03 1e+03) 0.0 0.0)))

(fn GenerateShockAttackXPosition
  (bind _returnvalue (Transformation|GetActorTransform))
  (bind _shock_attack_spawned_count (Variables|Attack-ShockAttack|GetShock%20Attack%20Spawned%20Count))
  (bind _location (Math|Transform|BreakTransform _returnvalue))
  (if (Variables|ForFlipping|GetLook%20Left)
    (return (+ (.x _location) (* _shock_attack_spawned_count 80)))
    (else
      (return (+ (.x _location) (* _shock_attack_spawned_count -80))))))