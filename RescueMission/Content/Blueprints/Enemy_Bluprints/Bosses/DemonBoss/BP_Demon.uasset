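; BP_Demon is a Paper2D demon boss that chases the player and attacks with an axe cleave.
; It extends a parent enemy's BeginPlay and Tick, using a state enum to switch from walking to attacking near the player.
; Cleaves use timed delays to spawn a directional slash effect, while sprite overlaps during that flipbook also deal damage.
; Taking damage plays hit or death flipbooks, with death calling BossDied.
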(event OnComponentBeginOverlap(Sprite)
  (params (OverlappedComponent :type Primitive%20Component%20Object%20Reference) (OtherActor :type Actor%20Object%20Reference) (OtherComp :type Primitive%20Component%20Object%20Reference) (OtherBodyIndex :type Integer) (bFromSweep :type Boolean) (SweepResult :type Hit%20Result%20Structure%20%28by%20ref%29))
  (if (and (== (Utilities|GetClass OtherActor) "/Game/Blueprints/Chracter_Blueprint/Paper2DCharacter.Paper2DCharacter_C") (== (Class|PaperFlipbookComponent|GetFlipbook (Variables|Default|GetSprite)) "/Game/Assets/Enemy_Assets/boss_demon_slime_FREE_v1_0/individual_sprites/03_demon_cleave/demon_cleave.demon_cleave"))
    (Game|Damage|ApplyDamage OtherActor (Variables|Default|GetDamage%20Amount) 0 0)))

(event EventBeginPlay
  (Variables|Default|SetHealth 6e+03)
  (Utilities|FlowControl|Sequence
    (:then_0
      (Variables|Default|SetPlayer%20Detection%20Range 5.5e+02))
    (:then_1
      (CallFunction|CalculateDistancetoPlayer)
      (if (Variables|Default|GetIs%20Detecting%20Player)
        (Variables|Default|SetCurrent%20State "NewEnumerator0")
        (else
          (Variables|Default|SetCurrent%20State "NewEnumerator3"))))
    (:then_2
      (|CallParentFunction))))

(event Collision|EventActorBeginOverlap
  (params (OtherActor :type Actor%20Object%20Reference)))

(event EventTick
  (params (DeltaSeconds :type Float%20%28single-precision%29))
  (Variables|Default|SetDelta%20Seconds DeltaSeconds)
  (if (> (Variables|Default|GetHealth) 0.0)
    (bind _new_look_left (CallFunction|Flip (Variables|Default|GetLook%20Left)))
    (Variables|Default|SetLook%20Left _new_look_left)
    (|CallParentFunction (Variables|Default|GetDelta%20Seconds))))

(event EventMovement
  (if (Utilities|Enum|Equal(Enum) (Variables|Default|GetCurrent%20State) "NewEnumerator0")
    (if (and (> (Math|Float|Absolute(Float) (CallFunction|GetXDistancetoPlayer)) 2.6e+02) (> (CallFunction|GetZDistancetoPlayer) -1.5e+02))
      (Sprite|SetFlipbook (Variables|Default|GetSprite) "/Game/Assets/Enemy_Assets/boss_demon_slime_FREE_v1_0/individual_sprites/02_demon_walk/demon_walk.demon_walk")
      (if (< (CallFunction|GetXDistancetoPlayer) 0.0)
        (Pawn|Input|AddMovementInput "0.500000, 0, 0" 1.0 false)
        (else
          (Pawn|Input|AddMovementInput "-0.500000, 0, 0" 1.0 false)))
      (else
        (Variables|Default|SetCurrent%20State "NewEnumerator1")))))

(event EventAttackAction
  (bind _returnvalue (Transformation|GetActorLocation))
  (Sprite|SetFlipbook (Variables|Default|GetSprite) "/Game/Assets/Enemy_Assets/boss_demon_slime_FREE_v1_0/individual_sprites/03_demon_cleave/demon_cleave.demon_cleave")
  (Utilities|FlowControl|Delay 1.7)
  (if (Variables|Default|GetLook%20Left)
    (Game|SpawnActorfromClass "/Game/Blueprints/Other/BP_DemonSlashEffect.BP_DemonSlashEffect_C" (Math|Transform|MakeTransform (Math|Vector|MakeVector (+ (.x _returnvalue) -2.6e+02) (.y _returnvalue) (.z _returnvalue)) "0, 0, 0" "1.000000,1.000000,1.000000") "Undefined" 0 0)
    (else
      (Game|SpawnActorfromClass "/Game/Blueprints/Other/BP_DemonSlashEffect.BP_DemonSlashEffect_C" (Math|Transform|MakeTransform (Math|Vector|MakeVector (+ (.x _returnvalue) 2.6e+02) (.y _returnvalue) (.z _returnvalue)) "0, 0, 0" "1.000000,1.000000,1.000000") "Undefined" 0 0)))
  (Audio|PlaySound2D "/Game/MusicAndSfx/BossMusicAndSFX/BossSFX_2/axe_swing.axe_swing" 1.0 1.0 0.0 0 0)
  (Utilities|FlowControl|Delay (- (Class|PaperFlipbookComponent|GetFlipbookLength (Variables|Default|GetSprite)) 2.0))
  (Variables|Default|SetCurrent%20State "NewEnumerator0"))

(event Game|Damage|EventAnyDamage
  (params (Damage :type Float%20%28single-precision%29) (DamageType :type Damage%20Type%20Object%20Reference) (InstigatedBy :type Controller%20Object%20Reference) (DamageCauser :type Actor%20Object%20Reference))
  (bind _sprite (Variables|Default|GetSprite))
  (bind _sprite_2 (Variables|Default|GetSprite))
  (bind _sprite_3 (Variables|Default|GetSprite))
  (if (> (Variables|Default|GetHealth) 0.0)
    (CallFunction|DecreaseHealth Damage)
    (if (not (Variables|Default|GetisTakeHitAnimationPlaying))
      (Sprite|SetFlipbook _sprite_3 "/Game/Assets/Enemy_Assets/boss_demon_slime_FREE_v1_0/individual_sprites/04_demon_take_hit/demon_take_hit.demon_take_hit")
      (Variables|Default|SetisTakeHitAnimationPlaying true)
      (Utilities|FlowControl|Delay (Class|PaperFlipbookComponent|GetFlipbookLength _sprite_3))
      (Variables|Default|SetisTakeHitAnimationPlaying false)
      (if (not (> (Variables|Default|GetHealth) 0.0))
        (Sprite|SetFlipbook _sprite_2 "/Game/Assets/Enemy_Assets/boss_demon_slime_FREE_v1_0/individual_sprites/05_demon_death/demon_death.demon_death")
        (Components|Timeline|SetLooping _sprite_2 false)
        (Collision|SetCollisionEnabled (Variables|Default|GetCapsuleComponent) "NoCollision")
        (Default|CallBossDied 1)))
    (else
      (Sprite|SetFlipbook _sprite "/Game/Assets/Enemy_Assets/boss_demon_slime_FREE_v1_0/individual_sprites/05_demon_death/demon_death.demon_death")
      (Components|Timeline|SetLooping _sprite false)
      (Default|CallBossDied 1))))

(fn ConstructionScript
  (|CallParentFunction))