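; Jumper enemy Blueprint that hops at timed intervals, with its health and damage stats set on BeginPlay before calling the parent.
; Tick accumulates time until it exceeds JumpInSeconds, then launches the character with random upward and slightly positive-biased X velocity.
; The parent Tick runs only on jump frames.
; Player range and side-check helper functions are defined but not called in these graphs.
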(event EventBeginPlay
  (Variables|Default|SetBase%20Damage 1e+01)
  (Variables|Default|SetDamage%20Duration 1.5)
  (Variables|Default|SetHealth 5e+01)
  (|CallParentFunction))

(event Collision|EventActorBeginOverlap
  (params (OtherActor :type Actor%20Object%20Reference)))

(event EventTick
  (params (DeltaSeconds :type Float%20%28single-precision%29))
  (Variables|Default|SetDelta%20Seconds DeltaSeconds)
  (bind _output_get (Variables|Default|SetJump%20Timer (+ (Variables|Default|GetDelta%20Seconds) (Variables|Default|GetJump%20Timer))))
  (if (not (<= _output_get (Variables|Default|GetJump%20In%20Seconds)))
    (Character|LaunchCharacter (Math|Vector|MakeVector (+ (Math|Random|RandomFloatinRange -5e+02 5e+02) 1e+02) 0.0 (Math|Random|RandomFloatinRange 5e+02 6e+02)) false false)
    (Variables|Default|SetJump%20Timer 0.0)
    (|CallParentFunction (Variables|Default|GetDelta%20Seconds))))

(fn ConstructionScript
  (|CallParentFunction))

(fn PlayerDetector
  (params (Range :type Float%20%28double-precision%29) (Player%20Location :type Vector) (Enemy%20Location :type Vector))
  (if (< (Math|Vector|Distance(Vector) Player%20Location Enemy%20Location) Range)
    (return true)
    (else
      (return false))))

(fn IsPlayeronRight
  (params (Player%20Location :type Vector) (Enemy%20Location :type Vector))
  (if (< (- (.x Player%20Location) (.x Enemy%20Location)) 0.0)
    (return false)
    (else
      (return true))))