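; Paper2D suicide-bomber enemy that homes in on the player while detecting them, then explodes after a short countdown.
; Tick updates player distance, halts movement when undetected, and otherwise runs the timer and sets the FlyingMovement homing target.
; On expiry it plays the explosion flipbook, damages Metroid once if still detecting, then destroys itself.
; Capsule and sprite contact handlers repeat the explosion but require DamageOnce to be already true, so initial contact does not detonate it.
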(event OnComponentHit(Sprite)
  (params (HitComponent :type Primitive%20Component%20Object%20Reference) (OtherActor :type Actor%20Object%20Reference) (OtherComp :type Primitive%20Component%20Object%20Reference) (NormalImpulse :type Vector :default "0, 0, 0") (Hit :type Hit%20Result%20Structure%20%28by%20ref%29))
  (bind _sprite (Variables|Default|GetSprite))
  (Utilities|Casting|CastToPaper2DCharacter OtherActor
    (:then
      _)
    (:CastFailed
      (Utilities|Casting|CastToBP_Mutated_Character OtherActor)))
  (if (Variables|Default|GetDamage%20Once)
    (Sprite|SetFlipbook _sprite "/Game/Assets/Enemy_Assets/PackMonsters/explode/Monster6Pack2.Monster6Pack2")
    (Game|Damage|ApplyDamage (Variables|Default|GetMetroid) (Variables|Default|GetBase%20Damage) 0 0)
    (Variables|Default|SetDamage%20Once true)
    (Utilities|FlowControl|Delay (Class|PaperFlipbookComponent|GetFlipbookLength _sprite))
    (Actor|DestroyActor)))

(event OnComponentBeginOverlap(CapsuleComponent)
  (params (OverlappedComponent :type Primitive%20Component%20Object%20Reference) (OtherActor :type Actor%20Object%20Reference) (OtherComp :type Primitive%20Component%20Object%20Reference) (OtherBodyIndex :type Integer) (bFromSweep :type Boolean) (SweepResult :type Hit%20Result%20Structure%20%28by%20ref%29))
  (bind _sprite (Variables|Default|GetSprite))
  ;[1 1 1] Explosion on Collision
  (Utilities|Casting|CastToPaper2DCharacter OtherActor
    (:then
      _)
    (:CastFailed
      (Utilities|Casting|CastToBP_Mutated_Character OtherActor)))
  (if (Variables|Default|GetDamage%20Once)
    (Sprite|SetFlipbook _sprite "/Game/Assets/Enemy_Assets/PackMonsters/explode/Monster6Pack2.Monster6Pack2")
    (Game|Damage|ApplyDamage (Variables|Default|GetMetroid) (Variables|Default|GetBase%20Damage) 0 0)
    (Variables|Default|SetDamage%20Once true)
    (Utilities|FlowControl|Delay (Class|PaperFlipbookComponent|GetFlipbookLength _sprite))
    (Actor|DestroyActor)))

(event OnComponentBeginOverlap(Sprite)
  (params (OverlappedComponent :type Primitive%20Component%20Object%20Reference) (OtherActor :type Actor%20Object%20Reference) (OtherComp :type Primitive%20Component%20Object%20Reference) (OtherBodyIndex :type Integer) (bFromSweep :type Boolean) (SweepResult :type Hit%20Result%20Structure%20%28by%20ref%29))
  (bind _sprite (Variables|Default|GetSprite))
  (Utilities|Casting|CastToPaper2DCharacter OtherActor
    (:then
      _)
    (:CastFailed
      (Utilities|Casting|CastToBP_Mutated_Character OtherActor)))
  (if (Variables|Default|GetDamage%20Once)
    (Sprite|SetFlipbook _sprite "/Game/Assets/Enemy_Assets/PackMonsters/explode/Monster6Pack2.Monster6Pack2")
    (Game|Damage|ApplyDamage (Variables|Default|GetMetroid) (Variables|Default|GetBase%20Damage) 0 0)
    (Variables|Default|SetDamage%20Once true)
    (Utilities|FlowControl|Delay (Class|PaperFlipbookComponent|GetFlipbookLength _sprite))
    (Actor|DestroyActor)))

(event EventBeginPlay
  (|CallParentFunction)
  (Variables|Default|SetBase%20Damage 1e+01)
  (Variables|Default|SetDamage%20Once false)
  (Variables|Default|SetExplosion%20Time 0.1))

(event Collision|EventActorBeginOverlap
  (params (OtherActor :type Actor%20Object%20Reference)))

(event EventTick
  (params (DeltaSeconds :type Float%20%28single-precision%29))
  (bind _sprite (Variables|Default|GetSprite))
  ;[1 1 1] Follow Player When On Spesific Bounds + Explosion After 2 Seconds of Movement
  (CallFunction|CalculateDistancetoPlayer)
  (if (Variables|Default|GetIsDetectingPlayer)
    (CallFunction|CountDownExplosionTimer DeltaSeconds)
    (bind _aspaper_2dcharacter (Utilities|Casting|CastToPaper2DCharacter (Game|GetPlayerCharacter 0)))
    (Variables|/Script/Engine.ProjectileMovementComponent|SetHomingTargetComponent (Variables|Default|GetFlyingMovement) (Variables|/Script/Engine.Character|GetCapsuleComponent _aspaper_2dcharacter))
    (if (<= (Variables|Default|GetExplosion%20Time) 0.0)
      (Sprite|SetFlipbook _sprite "/Game/Assets/Enemy_Assets/PackMonsters/explode/Monster6Pack2.Monster6Pack2")
      (Utilities|FlowControl|Delay (Class|PaperFlipbookComponent|GetFlipbookLength _sprite))
      (if (and (Variables|Default|GetIsDetectingPlayer) (not (Variables|Default|GetDamage%20Once)))
        (Game|Damage|ApplyDamage (Variables|Default|GetMetroid) (Variables|Default|GetBase%20Damage) 0 0)
        (Variables|Default|SetDamage%20Once true))
      (Actor|DestroyActor))
    (else
      (Components|Movement|StopMovementImmediately (Variables|Default|GetFlyingMovement)))))

(fn ConstructionScript
  (|CallParentFunction))