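; Bringer of Death enemy, a flipbook-sprite character that walks, melees, casts spells at the player and dies at zero health.
; Tick sets range flags, picks a state, then runs it; casting spawns BringerCast_BP near the player.
; PlayerDetector ignores its Range input, returning true whenever X positions differ.
; Overlaps start or end player damage-over-time; Bullet_BP hits play a hurt flipbook without reducing Health.
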(event OnComponentHit(Sprite)
  (params (HitComponent :type Primitive%20Component%20Object%20Reference) (OtherActor :type Actor%20Object%20Reference) (OtherComp :type Primitive%20Component%20Object%20Reference) (NormalImpulse :type Vector :default "0, 0, 0") (Hit :type Hit%20Result%20Structure%20%28by%20ref%29))
  (bind _sprite (Variables|Default|GetSprite))
  ;[1 1 1] Hurt
  (Utilities|Casting|CastToBullet_BP OtherActor)
  (Variables|Default|SetCurrent%20State "NewEnumerator3")
  (Sprite|SetFlipbook _sprite (Variables|Default|GetHurtFlipbook))
  (Utilities|FlowControl|Delay (Class|PaperFlipbookComponent|GetFlipbookLength (Variables|Default|GetSprite)))
  (Variables|Default|SetCurrent%20State "NewEnumerator1")
  (Sprite|SetFlipbook _sprite (Variables|Default|GetIdleFlipbook)))

(event OnComponentBeginOverlap(Sprite)
  (params (OverlappedComponent :type Primitive%20Component%20Object%20Reference) (OtherActor :type Actor%20Object%20Reference) (OtherComp :type Primitive%20Component%20Object%20Reference) (OtherBodyIndex :type Integer) (bFromSweep :type Boolean) (SweepResult :type Hit%20Result%20Structure%20%28by%20ref%29))
  (bind _metroid (Variables|Default|GetMetroid))
  ;[1 1 1] Damage in interaction with the player
  (bind _playerref (Class|PlayerInterface|PlayerRef(Message) OtherActor))
  (Utilities|IsValid _playerref
    (:Is%20Valid
      _)
    (:Is%20Not%20Valid
      (bind _playerref_2 (Class|MutatedInterface|MutatedPlayerRef(Message) OtherActor))
      (Utilities|IsValid _playerref_2
        (:Is%20Valid
          _))))
  (if (Utilities|Enum|Equal(Enum) (Variables|Default|GetCurrent%20State) "NewEnumerator5")
    (Variables|/Game/Blueprints/Chracter_Blueprint/Paper2DCharacter.Paper2DCharacter_C|SetDamage%20Recieved _metroid (Variables|Default|GetBase%20Damage))
    (Variables|/Game/Blueprints/Chracter_Blueprint/Paper2DCharacter.Paper2DCharacter_C|SetDuration _metroid (Variables|Default|GetDamage%20Duration))
    (Default|Dot _playerref)))

(event OnComponentBeginOverlap(CapsuleComponent)
  (params (OverlappedComponent :type Primitive%20Component%20Object%20Reference) (OtherActor :type Actor%20Object%20Reference) (OtherComp :type Primitive%20Component%20Object%20Reference) (OtherBodyIndex :type Integer) (bFromSweep :type Boolean) (SweepResult :type Hit%20Result%20Structure%20%28by%20ref%29))
  (bind _metroid (Variables|Default|GetMetroid))
  ;[1 1 1] Comment
  (bind _playerref (Class|PlayerInterface|PlayerRef(Message) OtherActor))
  (Utilities|IsValid _playerref
    (:Is%20Valid
      _)
    (:Is%20Not%20Valid
      (bind _playerref_2 (Class|MutatedInterface|MutatedPlayerRef(Message) OtherActor))
      (Utilities|IsValid _playerref_2
        (:Is%20Valid
          _))))
  (Variables|/Game/Blueprints/Chracter_Blueprint/Paper2DCharacter.Paper2DCharacter_C|SetDamage%20Recieved _metroid (Variables|Default|GetBase%20Damage))
  (Variables|/Game/Blueprints/Chracter_Blueprint/Paper2DCharacter.Paper2DCharacter_C|SetDuration _metroid (Variables|Default|GetDamage%20Duration))
  (Default|Dot _playerref)
  (Default|StartDot _playerref))

(event OnComponentEndOverlap(CapsuleComponent)
  (params (OverlappedComponent :type Primitive%20Component%20Object%20Reference) (OtherActor :type Actor%20Object%20Reference) (OtherComp :type Primitive%20Component%20Object%20Reference) (OtherBodyIndex :type Integer))
  ;[1 1 1] Comment
  (bind _playerref (Class|PlayerInterface|PlayerRef(Message) OtherActor))
  (Utilities|IsValid _playerref
    (:Is%20Valid
      _)
    (:Is%20Not%20Valid
      (bind _playerref_2 (Class|MutatedInterface|MutatedPlayerRef(Message) OtherActor))
      (Utilities|IsValid _playerref_2
        (:Is%20Valid
          _))))
  (Default|EndDot _playerref))

(event OnComponentEndOverlap(Sprite)
  (params (OverlappedComponent :type Primitive%20Component%20Object%20Reference) (OtherActor :type Actor%20Object%20Reference) (OtherComp :type Primitive%20Component%20Object%20Reference) (OtherBodyIndex :type Integer))
  ;[1 1 1] Damage in interaction with the player
  (bind _playerref (Class|PlayerInterface|PlayerRef(Message) OtherActor))
  (Utilities|IsValid _playerref
    (:Is%20Valid
      _)
    (:Is%20Not%20Valid
      (bind _playerref_2 (Class|MutatedInterface|MutatedPlayerRef(Message) OtherActor))
      (Utilities|IsValid _playerref_2
        (:Is%20Valid
          _))))
  (Default|EndDot _playerref))

(event Custom|Melee%20Attack
  ;[1 1 1] Melee Attack
  (CallFunction|RotateTowardsPlayer)
  (Variables|Default|SetBase%20Damage 1.0)
  (Sprite|SetFlipbook (Variables|Default|GetSprite) (Variables|Default|GetAttackFlipbook)))

(event Custom|Death
  ;[1 1 1] Death
  (Sprite|SetFlipbook (Variables|Default|GetSprite) (Variables|Default|GetDeathFlipbook))
  (Utilities|FlowControl|Delay (CallFunction|GetSpriteFlipbookLength (Variables|Default|GetDeathFlipbook)))
  (Actor|DestroyActor))

(event Custom|Casting%20Attack
  (bind _returnvalue (Game|GetPlayerCharacter 0))
  (bind _returnvalue_2 (Transformation|GetActorTransform _returnvalue))
  ;[1 1 1] Spell Attack
  (CallFunction|RotateTowardsPlayer)
  (Sprite|SetFlipbook (Variables|Default|GetSprite) (Variables|Default|GetCastFlipbook))
  (Game|SpawnActorfromClass "/Game/Blueprints/Bullet_and_Impact_Blueprint/Cast/BringerCast_BP.BringerCast_BP_C" (Math|Transform|MakeTransform (Math|Vector|MakeVector (.x (.location _returnvalue_2)) (.y (.location _returnvalue_2)) (+ (.z (.location _returnvalue_2)) (Math|Random|RandomFloatinRange -5e+01 5e+01))) (.rotation _returnvalue_2) (.scale _returnvalue_2)) "AdjustIfPossibleButDontSpawnIfColliding" 0 0)
  (Utilities|FlowControl|Delay 1.0))

(event Custom|Walk
  ;[1 1 1] Walk
  (CallFunction|RotateTowardsPlayer)
  (Sprite|SetFlipbook (Variables|Default|GetSprite) (Variables|Default|GetWalkFlipbook))
  (Pawn|Input|AddMovementInput (Transformation|GetActorLocation (Game|GetPlayerCharacter 0)) 1.0 false))

(event Custom|Range%20Decider
  (bind _returnvalue (Game|GetPlayerCharacter 0))
  (bind _self self)
  (bind _returnvalue_2 (Transformation|GetActorLocation _returnvalue))
  (bind _returnvalue_3 (Transformation|GetActorLocation _self))
  ;[1 1 1] Setting the booleans according the distance of the player
  (bind _player_in_range (CallFunction|PlayerDetector (Variables|Default|GetMelee%20Range) _returnvalue_2 _returnvalue_3))
  (Variables|Default|SetIs%20Player%20In%20Melee%20Range _player_in_range)
  (bind _player_in_range_2 (CallFunction|PlayerDetector (Variables|Default|GetCast%20Range) _returnvalue_2 _returnvalue_3))
  (Variables|Default|SetIs%20Player%20In%20Cast%20Range _player_in_range_2)
  (bind _player_in_range_3 (CallFunction|PlayerDetector (Variables|Default|GetWalk%20Range) _returnvalue_2 _returnvalue_3))
  (Variables|Default|SetIs%20Player%20In%20Walk%20Range _player_in_range_3))

(event Custom|State%20Setter
  ;[1 1 1] State Setter
  (if (Variables|Default|GetIs%20Player%20In%20Melee%20Range)
    (Variables|Default|SetCurrent%20State "NewEnumerator5")
    (elif (Variables|Default|GetIs%20Player%20In%20Walk%20Range)
      (Variables|Default|SetCurrent%20State "NewEnumerator2")
      (elif (Variables|Default|GetIs%20Player%20In%20Cast%20Range)
        (Variables|Default|SetCurrent%20State "NewEnumerator0")
        (else
          (Variables|Default|SetCurrent%20State "NewEnumerator1"))))))

(event Collision|EventActorBeginOverlap
  (params (OtherActor :type Actor%20Object%20Reference)))

(event EventTick
  (params (DeltaSeconds :type Float%20%28single-precision%29))
  ;[1 1 1] State Machine in Event tick
  (|CallParentFunction DeltaSeconds)
  (if (== (Variables|Default|GetHealth) 0.0)
    (CallFunction|Death)
    (else
      (Variables|Default|SetBase%20Damage 0.0)
      (CallFunction|RangeDecider)
      (CallFunction|StateSetter)
      (switch Utilities|FlowControl|Switch|SwitchonBringerEnemy_Enum (Variables|Default|GetCurrent%20State)
        (:NewEnumerator0
          (CallFunction|Walk))
        (:NewEnumerator2
          (CallFunction|CastingAttack))
        (:NewEnumerator4
          (CallFunction|Death))
        (:NewEnumerator5
          (CallFunction|MeleeAttack))))))

(event EventBeginPlay
  (Variables|Default|SetCurrent%20State "NewEnumerator1")
  (Variables|Default|SetBase%20Damage 1.0)
  (Variables|Default|SetDamage%20Duration 1.5)
  (Variables|Default|SetHealth 5e+01)
  (Variables|Default|SetisMovingRight false)
  (|CallParentFunction))

(fn ConstructionScript
  (|CallParentFunction))

(fn PlayerDetector
  (params (Range :type Float%20%28double-precision%29) (Player%20Location :type Vector) (Enemy%20Location :type Vector))
  (if (< 0.0 (Math|Float|Absolute(Float) (- (.x Player%20Location) (.x Enemy%20Location))))
    (return true)
    (else
      (return false))))