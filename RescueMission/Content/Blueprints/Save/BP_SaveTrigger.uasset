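; Save point trigger that saves the game when the player character overlaps it.
; A Sequence on overlap starts the feedback branch, then calls Save on GameMode_BP without waiting for its delays.
; The feedback runs only if the player's Health is not 100: a pitched-up startup sound, camera fade to black, brief Save_Widget display, then fade back in.
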(event EventBeginPlay)

(event Collision|EventActorBeginOverlap
  (params (OtherActor :type Actor%20Object%20Reference))
  (bind _returnvalue (Game|GetPlayerCharacter 0))
  (if (== OtherActor _returnvalue)
    (Utilities|FlowControl|Sequence
      (:then_0
        (bind _aspaper_2dcharacter (Utilities|Casting|CastToPaper2DCharacter _returnvalue))
        (if (not (== (Variables|/Game/Blueprints/Chracter_Blueprint/Paper2DCharacter.Paper2DCharacter_C|GetHealth _aspaper_2dcharacter) 1e+02))
          (Audio|PlaySound2D "/Game/MusicAndSfx/Microsoft_Windows_98_Startup_Sound.Microsoft_Windows_98_Startup_Sound" 0.5 2.5 0.0 0 0)
          (CameraFades|StartCameraFade :self (Game|GetPlayerCameraManager 0) :ToAlpha 1.0 :Duration 1.0 :bHoldWhenFinished true)
          (Utilities|FlowControl|Delay 1.0)
          (bind _returnvalue_2 (UserInterface|CreateWidget "/Game/Assets/UI_Assets/Widgets/Save_Widget.Save_Widget_C"))
          (UserInterface|Viewport|AddtoViewport _returnvalue_2 0)
          (Utilities|FlowControl|Delay 0.5)
          (Widget|RemovefromParent _returnvalue_2)
          (CameraFades|StartCameraFade :self (Game|GetPlayerCameraManager 0) :FromAlpha 1.0 :Duration 1.0)))
      (:then_1
        (bind _asgame_mode_bp (Utilities|Casting|CastToGameMode_BP (Game|GetGameMode)))
        (Default|Save _asgame_mode_bp)))))

(event EventTick
  (params (DeltaSeconds :type Float%20%28single-precision%29)))

(fn ConstructionScript)