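; Game music manager actor that plays soundtracks on an audio component from BeginPlay and steps through separate layer and boss track lists.
; Each advance stops playback and remembers the outgoing track, so ContinuePreviousMusic can swap back to it.
; EndBossMusic sets the "Music State" audio parameter, waits briefly, then restores the previous track.
; EndCurrentBossMusic is an empty stub, and a debug print remains in ContinuePreviousMusic.
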(event Custom|End%20Boss%20Music
  (Effects|Components|ParticleSystem|SetIntParameter (Variables|Components|GetAudioComponent) "Music State" 1)
  (Utilities|FlowControl|Delay 5.0)
  (CallFunction|ContinuePreviousMusic))

(event EventBeginPlay
  (Audio|Components|Audio|Play (Variables|Components|GetAudioComponent) 0.0))

(event EventTick
  (params (DeltaSeconds :type Float%20%28single-precision%29)))

(fn ConstructionScript)

(fn StopCurrentMusic
  (Audio|Components|Audio|Stop (Variables|Components|GetAudioComponent)))

(fn PlayNextLayerSoundtrack
  (CallFunction|StopCurrentMusic)
  (Variables|Default|SetPrevious%20Music (Variables|Default|GetCurrent%20Music))
  (if (< (+ (Variables|Default|GetCurrent%20Layer%20Soundtrack%20Index) 1) (Utilities|Array|Length (Variables|Default|GetLayer%20Soundtrack%20List)))
    (bind _result (Math|Integer|IncrementInt (Variables|Default|GetCurrent%20Layer%20Soundtrack%20Index))
      (:%20%20
        (Audio|Components|Audio|SetSound (Variables|Components|GetAudioComponent) (Utilities|Array|Get(acopy) (Variables|Default|GetLayer%20Soundtrack%20List) _result))
        (Audio|Components|Audio|Play (Variables|Components|GetAudioComponent) 0.0)
        (Variables|Default|SetCurrent%20Music (Utilities|Array|Get(acopy) (Variables|Default|GetLayer%20Soundtrack%20List) _result))))))

(fn PlayNextBossSoundtrack
  (CallFunction|StopCurrentMusic)
  (Variables|Default|SetPrevious%20Music (Variables|Default|GetCurrent%20Music))
  (if (< (+ (Variables|Default|GetCurrent%20Boss%20Soundtrack%20Index) 1) (Utilities|Array|Length (Variables|Default|GetBoss%20Soundtrack%20List)))
    (bind _result (Math|Integer|IncrementInt (Variables|Default|GetCurrent%20Boss%20Soundtrack%20Index))
      (:%20%20
        (Audio|Components|Audio|SetSound (Variables|Components|GetAudioComponent) (Utilities|Array|Get(acopy) (Variables|Default|GetBoss%20Soundtrack%20List) _result))
        (Audio|Components|Audio|Play (Variables|Components|GetAudioComponent) 0.0)
        (Variables|Default|SetCurrent%20Music (Utilities|Array|Get(acopy) (Variables|Default|GetBoss%20Soundtrack%20List) _result))))))

(fn ContinuePreviousMusic
  (CallFunction|StopCurrentMusic)
  (LocalVariables|SetLocal%20Previous%20Music (Variables|Default|GetCurrent%20Music))
  (Variables|Default|SetCurrent%20Music (Variables|Default|GetPrevious%20Music))
  (Variables|Default|SetPrevious%20Music (LocalVariables|GetLocal%20Previous%20Music))
  (Audio|Components|Audio|SetSound (Variables|Components|GetAudioComponent) (Variables|Default|GetCurrent%20Music))
  (Audio|Components|Audio|Play (Variables|Components|GetAudioComponent) 0.0)
  (Development|PrintString "Hello"))

(fn EndCurrentBossMusic)